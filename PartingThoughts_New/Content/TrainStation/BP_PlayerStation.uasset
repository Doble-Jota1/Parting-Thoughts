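; Player pawn for the train station level, with a book menu and a scripted parting scene.
; After a delay it raises a spawned book into view and traces the cursor against it: clicks either load a level or show a ticket.
; Unless IsBook locks input, Space walks it along a spline to the first point, where timelines align the view and raise an arm, then Niagara pauses and a title card appears.
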(event Custom|ShowBook
  (bind _returnvalue (Transformation|GetActorForwardVector))
  (bind _sphere (Variables|Default|GetSphere))
  (bind _returnvalue_2 (Transformation|GetWorldTransform _sphere))
  (bind _returnvalue_3 (* _returnvalue 1e+02))
  (bind _returnvalue_4 (- (.location _returnvalue_2) "0.000000,0.000000,100.000000"))
  (bind _returnvalue_5 (- _returnvalue_4 _returnvalue_3))
  (Variables|Default|SetbIsBook true)
  (bind _returnvalue_6 (Game|SpawnActorfromClass "/Game/TrainStation/BP_Book.BP_Book_C" (Math|Transform|MakeTransform _returnvalue_5 "0, 0, 0" "0.060000,0.060000,0.060000") "AlwaysSpawn" "MultiplyWithRoot" 0 0))
  (bind _output_get (Variables|Default|SetBook _returnvalue_6))
  (Transformation|AttachComponentToComponent _output_get (Variables|Default|GetSphere) "None" "KeepWorld" "KeepRelative" "KeepWorld" true)
  (bind _alpha (Timeline|BookTakeOut PlayFromStart)
    (:Update
      (Transformation|SetActorLocation (Variables|Default|GetBook) (Math|Vector|Lerp(Vector) _returnvalue_5 (.location _returnvalue_2) _alpha) false false))
    (:Finished
      (Variables|/Script/Engine.PlayerController|SetbShowMouseCursor (Game|GetPlayerController 0) true)
      (Actor|Tick|SetActorTickEnabled true))))

(event Custom|BookTrace
  (bind _returnvalue (Game|GetPlayerController 0))
  (bind (_worldlocation _worlddirection) (Game|Player|ConvertMouseLocationToWorldSpace _returnvalue))
  (bind _outhit (Collision|LineTraceForObjects _worldlocation (+ _worldlocation (* _worlddirection 5e+02)) (Utilities|Array|MakeArray "ObjectTypeQuery8") true 0 "None"))
  (Variables|Default|SetHit%20Component (.HitComponent (Collision|BreakHitResult _outhit))))

(event Custom|RaiseArm
  (Utilities|FlowControl|Sequence
    (:then_0
      (bind _alpha (Timeline|Raise PlayFromStart)
        (:Update
          (Transformation|SetRelativeLocationAndRotation (Variables|Default|GetLiftingArm) (Math|Vector|Lerp(Vector) "0.300000,13.000000,-27.000000" "27.000000,14.000000,-13.000000" _alpha) (Math|Rotator|Lerp(Rotator) "0.700000,-99.000000,-19.000000" "13.500000,-105.000000,-18.000000" _alpha true) false false))))
    (:then_1
      (Utilities|FlowControl|Delay 0.6)
      (Components|Animation|PlayAnimation (Variables|Default|GetLiftingArm) "/Game/TrainStation/Arm_Raise.Arm_Raise" false))))

(event Custom|Parting
  (bind _returnvalue (Game|GetPlayerController 0))
  (bind _returnvalue_2 (Transformation|GetActorLocation))
  (bind _destination (Variables|Default|GetDestination))
  (Variables|Default|SetbIsBook true)
  (bind _output_get (Variables|Default|SetStartingRotation (Pawn|GetControlRotation _returnvalue :!class /Script/Engine.Controller)))
  (bind _output_get_2 (Variables|Default|SetStartingLocation _returnvalue_2))
  (bind _alpha (Timeline|Orient PlayFromStart)
    (:Update
      (Pawn|SetControlRotation _returnvalue (Math|Rotator|Lerp(Rotator) _output_get "3.500000,-18.000000,0.000000" _alpha true))
      (Transformation|SetActorLocation (Math|Vector|Lerp(Vector) _output_get_2 (Math|Vector|MakeVector (.x _destination) (.y _destination) (.Z (Math|Vector|BreakVector _returnvalue_2))) _alpha) false false))
    (:Finished
      (Utilities|FlowControl|Delay 0.1)
      (CallFunction|RaiseArm)
      (Utilities|FlowControl|Delay 4.0)
      (bind _returnvalue_3 (Actor|GetActorOfClass "/Script/Niagara.NiagaraActor"))
      (Class|NiagaraComponent|SetPaused (Variables|/Script/Niagara.NiagaraActor|GetNiagaraComponent _returnvalue_3) true)
      (Utilities|FlowControl|Delay 2.0)
      (UserInterface|Viewport|AddtoViewport (Variables|Default|GetTitleCard) 0))))

(event Input|EnhancedActionEvents|EnhancedInputActionIA_Space
  (params (ActionValue :type Boolean) (ElapsedSeconds :type Float%20%28double-precision%29) (TriggeredSeconds :type Float%20%28double-precision%29) (InputAction :type Input%20Action%20Object%20Reference :default "/Game/Blueprints/Input/IA_Space.IA_Space"))
  (bind _returnvalue (Transformation|GetActorLocation))
  (if (not (Variables|Default|GetbIsBook))
    (Pawn|Input|AddMovementInput (Spline|FindDirectionClosesttoWorldLocation (Variables|Default|GetSpline) _returnvalue "World") -0.6 false)
    (if (< (Class|KismetMathLibrary|VectorDistanceSquared (Variables|Default|GetDestination) _returnvalue) (Variables|Default|GetThreshold))
      (CallFunction|Parting))))

(event Input|EnhancedActionEvents|EnhancedInputActionIA_LeftClick
  (params (ActionValue :type Boolean) (ElapsedSeconds :type Float%20%28double-precision%29) (TriggeredSeconds :type Float%20%28double-precision%29) (InputAction :type Input%20Action%20Object%20Reference :default "/Game/Blueprints/Input/IA_LeftClick.IA_LeftClick"))
  (:Completed
    (bind _hit_component (Variables|Default|GetHit%20Component)
      (:then
        (bind _bhastag (CallFunction|HasTag _hit_component "Empty"))
        (if _bhastag
          (bind _asbp_parting_game_instance (Utilities|Casting|CastToBP_PartingGameInstance (Game|GetGameInstance)))
          (Default|LoadLevel _asbp_parting_game_instance "/Game/Scene1/FractalPath.FractalPath")
          (else
            (UserInterface|Viewport|AddtoViewport (Variables|Default|GetTicket) 0))))
      (:else))))

(event Input|EnhancedActionEvents|EnhancedInputActionIA_Look
  (params (ActionValue :type Vector%202D%20Structure) (ElapsedSeconds :type Float%20%28double-precision%29) (TriggeredSeconds :type Float%20%28double-precision%29) (InputAction :type Input%20Action%20Object%20Reference :default "/Game/Blueprints/Input/IA_Look.IA_Look"))
  (if (not (Variables|Default|GetbIsBook))
    (Pawn|Input|AddControllerYawInput (.x ActionValue))
    (Pawn|Input|AddControllerPitchInput (.y ActionValue))))

(event Input|EnhancedActionEvents|EnhancedInputActionIA_Esc
  (params (ActionValue :type Boolean) (ElapsedSeconds :type Float%20%28double-precision%29) (TriggeredSeconds :type Float%20%28double-precision%29) (InputAction :type Input%20Action%20Object%20Reference :default "/Game/Blueprints/Input/IA_Esc.IA_Esc"))
  (bind _ticket (Variables|Default|GetTicket))
  (:Completed
    (if (UserInterface|Viewport|IsinViewport _ticket)
      (Widget|RemovefromParent _ticket))))

(event EventBeginPlay
  (Utilities|FlowControl|Sequence
    (:then_0
      (bind _returnvalue (Actor|GetActorOfClass "/Game/Scene1/BP_Spline.BP_Spline_C"))
      (bind _output_get (Variables|Default|SetSpline (Variables|/Game/Scene1/BP_Spline.BP_Spline_C|GetSpline _returnvalue)))
      (Transformation|SetActorLocation (Spline|FindLocationClosesttoWorldLocation _output_get (Transformation|GetActorLocation) "World") false false)
      (Variables|Default|SetDestination (Spline|GetLocationatSplinePoint _output_get 0 "World")))
    (:then_1
      (bind _returnvalue_2 (UserInterface|CreateWidget "/Game/TrainStation/WB_TitleCard.WB_TitleCard_C"))
      (Variables|Default|SetTitleCard _returnvalue_2)
      (bind _returnvalue_3 (UserInterface|CreateWidget "/Game/Book/WBP_Ticket.WBP_Ticket_C"))
      (Variables|Default|SetTicket _returnvalue_3)
      (Utilities|FlowControl|Delay 8.0)
      (CallFunction|ShowBook))))

(event EventTick
  (params (DeltaSeconds :type Float%20%28single-precision%29))
  (Utilities|FlowControl|Sequence
    (:then_0
      (CallFunction|BookTrace))))

(fn ConstructionScript)

(fn HasTag
  (params (Component :type Actor%20Component%20Object%20Reference) (Tag :type Name))
  (for _array_element (Variables|/Script/Engine.ActorComponent|GetComponentTags Component)
    (if (== _array_element Tag)
      (return true)))
  (return false))