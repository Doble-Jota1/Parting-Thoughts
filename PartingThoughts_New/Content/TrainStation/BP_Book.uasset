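; Book actor in the TrainStation folder that plays a one-shot, staggered animation when play begins.
; After a short delay, the skeletal mesh plays the outer book sequence without looping.
; Three page components then play once each, started one after another by brief delays to offset their motion.
; All timing comes from a single Delay chain on BeginPlay, with no other logic.
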(event EventBeginPlay
  (Utilities|FlowControl|Delay 0.5)
  (Components|Animation|PlayAnimation (Variables|Default|GetSkeletalMesh) "/Game/Book/BookOuter_Skeleton_Sequence.BookOuter_Skeleton_Sequence" false)
  (Utilities|FlowControl|Delay 0.3)
  (Audio|Components|Audio|Play (Variables|Default|GetPage) false)
  (Utilities|FlowControl|Delay 0.1)
  (Audio|Components|Audio|Play (Variables|Default|GetPage1) false)
  (Utilities|FlowControl|Delay 0.1)
  (Audio|Components|Audio|Play (Variables|Default|GetPage2) false))

(fn ConstructionScript)