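; Scene 1 player character that walks along splines while Space is held, with smoothed look input and an intro camera pan.
; View yaw is clamped to the active spline; at junctions, gaze direction picks the branch and a timeline blends the limits.
; The MM event frees yaw and moves the Munin figure along its own spline, optionally pacing it to the player.
; Distance checks teleport both back or load the next scene.
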(event Custom|TransitionSplines
  (params (Old :type Spline%20Component%20Object%20Reference) (New :type Spline%20Component%20Object%20Reference))
  (bind _returnvalue (Game|GetPlayerCameraManager 0))
  (bind _returnvalue_2 (Transformation|GetActorLocation))
  (bind _constrait (Variables|Default|GetConstrait))
  (Utilities|FlowControl|Sequence
    (:then_0
      (bind _alpha (Timeline|Transit Stop)
        (:Update
          (Variables|/Script/Engine.PlayerCameraManager|SetViewYawMax _returnvalue (+ (Math|Float|Lerp (stale _output_get) (stale _output_get_2) _alpha) _constrait))
          (Variables|/Script/Engine.PlayerCameraManager|SetViewYawMin _returnvalue (- (Math|Float|Lerp (stale _output_get) (stale _output_get_2) _alpha) _constrait)))
        (:Finished
          (Variables|Default|SetbInTransition false))))
    (:then_1
      (bind _output_get (Variables|Default|SetOld (.yaw (Math|Rotator|MakeRotfromX (Spline|FindDirectionClosesttoWorldLocation Old _returnvalue_2 "World")))))
      (bind _output_get_2 (Variables|Default|SetNew (.yaw (Math|Rotator|MakeRotfromX (Spline|FindDirectionClosesttoWorldLocation New _returnvalue_2 "World")))))
      (Timeline|Transit PlayFromStart))))

(event Custom|MM
  (Audio|PlaySound2D "/Game/Music/2_MaggieMo.2_MaggieMo" 1.0 1.0 0.0 0 0)
  (Variables|Default|SetbIsMM true)
  (bind _outactors (Actor|GetAllActorsOfClasswithTag "/Game/2_Scene1/BP_Spline.BP_Spline_C" "Player"))
  (bind _output_get (Variables|Default|SetPlayerSpline (Utilities|Array|Get(acopy) _outactors)))
  (Variables|Default|SetActiveSpline (Variables|/Game/2_Scene1/BP_Spline.BP_Spline_C|GetSpline _output_get))
  (bind _outactors_2 (Actor|GetAllActorsOfClasswithTag "/Game/2_Scene1/BP_Spline.BP_Spline_C" "Figure"))
  (Variables|Default|SetFigureSpline (Utilities|Array|Get(acopy) _outactors_2))
  (Variables|/Script/Engine.CharacterMovementComponent|SetMaxWalkSpeed (Variables|Character|GetCharacterMovement) 6e+02)
  (bind _outactors_3 (Actor|GetAllActorsOfClasswithTag "/Script/Engine.StaticMeshActor" "MUN"))
  (Variables|Default|SetMunin (Utilities|Array|Get(acopy) _outactors_3))
  (Transformation|SetActorLocation (Variables|Default|GetMunin) (Math|Vector|MakeVector (.x (Spline|FindLocationClosesttoWorldLocation (Variables|/Game/2_Scene1/BP_Spline.BP_Spline_C|GetSpline (Variables|Default|GetFigureSpline)) (Transformation|GetActorLocation (Variables|Default|GetMunin)) "World")) (.y (Spline|FindLocationClosesttoWorldLocation (Variables|/Game/2_Scene1/BP_Spline.BP_Spline_C|GetSpline (Variables|Default|GetFigureSpline)) (Transformation|GetActorLocation (Variables|Default|GetMunin)) "World")) (.z (Transformation|GetActorLocation (Variables|Default|GetMunin)))) false false)
  (Variables|Default|SetTransition 0)
  (Utilities|FlowControl|Delay 2.0)
  (bind _returnvalue (UserInterface|CreateWidget "/Game/1_TrainStation/WB_TitleCard.WB_TitleCard_C"))
  (bind _output_get_2 (Variables|Default|SetTitleCard _returnvalue))
  (Variables|Default|SetbIsBook true)
  (CallFunction|NextCard "“I think it's time to go back” 
She says")
  (UserInterface|Viewport|AddtoViewport _output_get_2 0)
  (Utilities|FlowControl|Delay 4.0)
  (Widget|RemovefromParent _output_get_2)
  (Audio|Components|Audio|Stop (Variables|Default|GetCardSfx))
  (Variables|Default|SetbIsBook false)
  (Audio|PlaySound2D "/Game/Sfx/2_MaggieMoAmbience.2_MaggieMoAmbience" 4.0 1.0 0.0 0 0)
  (Audio|PlaySound2D "/Game/Music/2_MaggieMo.2_MaggieMo" 24.0 1.0 0.0 0 0))

(event Custom|SmoothLook
  (if (Variables|Default|GetbNotLooking)
    (bind _output_get (Variables|Default|SetSmoothedVector (Math|Vector2D|MakeVector2D (.x (Class|KismetMathLibrary|Vector2DInterpto (Variables|Default|GetSmoothedVector) (Math|Vector2D|MakeVector2D 0.0 0.0) (Utilities|Time|GetWorldDeltaSeconds) (Variables|Default|GetLookSmoothSpeed))) (.y (Class|KismetMathLibrary|Vector2DInterpto (Variables|Default|GetSmoothedVector) (Math|Vector2D|MakeVector2D 0.0 0.0) (Utilities|Time|GetWorldDeltaSeconds) (Variables|Default|GetLookSmoothSpeed))))))
    (Pawn|Input|AddControllerYawInput (.x _output_get))
    (Pawn|Input|AddControllerPitchInput (.y _output_get))))

(event Custom|Continue
  (bind _returnvalue (Transformation|GetActorLocation))
  (bind _returnvalue_2 (Transformation|GetActorLocation))
  (bind _munin (Variables|Default|GetMunin))
  (bind _munin_2 (Variables|Default|GetMunin))
  (bind _playerspline (Variables|Default|GetPlayerSpline))
  (bind _munin_3 (Variables|Default|GetMunin))
  (bind _munin_4 (Variables|Default|GetMunin))
  (bind _figurespline (Variables|Default|GetFigureSpline))
  (bind _figurespline_2 (Variables|Default|GetFigureSpline))
  (bind _returnvalue_3 (Transformation|GetActorLocation _munin_3))
  (bind _returnvalue_4 (Transformation|GetActorLocation _munin_2))
  (bind _z (Math|Vector|BreakVector _returnvalue))
  (bind _spline (Variables|/Game/2_Scene1/BP_Spline.BP_Spline_C|GetSpline _playerspline))
  (bind _spline_2 (Variables|/Game/2_Scene1/BP_Spline.BP_Spline_C|GetSpline _figurespline))
  (bind _spline_3 (Variables|/Game/2_Scene1/BP_Spline.BP_Spline_C|GetSpline _figurespline_2))
  (bind _returnvalue_5 (Spline|FindLocationClosesttoWorldLocation _spline_3 (Math|Vector|MakeVector 127557.135571 -57362.404877 1447.631975) "World"))
  (bind _returnvalue_6 (Spline|FindLocationClosesttoWorldLocation _spline _returnvalue_2 "World"))
  (Utilities|FlowControl|Gate true) ; enters at Open
)

(event Custom|RandomRotation
  (bind _returnvalue (Utilities|Time|SetTimerbyEvent (delegate Custom|RandomRotation) (Math|Random|RandomFloatinRange 0.5 4.0)))
  (Variables|Default|SetRotationTimerHandle _returnvalue)
  (Variables|Default|SetMuninSpeed (Math|Random|RandomFloatinRange 1.0 4.0)))

(event Custom|NextCard
  (params (InText :type Text))
  (bind _returnvalue (Audio|CreateSound2D "/Game/Sfx/Card.Card" 1.0 1.0 0.0 0))
  (bind _output_get (Variables|Default|SetCardSfx _returnvalue))
  (Audio|Components|Audio|Play _output_get 0.0)
  (Utilities|FlowControl|Delay 0.05)
  (Rendering|Components|TextRender|SetText (Variables|/Game/1_TrainStation/WB_TitleCard.WB_TitleCard_C|GetText (Variables|Default|GetTitleCard)) InText))

(event Input|EnhancedActionEvents|EnhancedInputActionIA_Space
  (params (ActionValue :type Boolean) (ElapsedSeconds :type Float%20%28double-precision%29) (TriggeredSeconds :type Float%20%28double-precision%29) (InputAction :type Input%20Action%20Object%20Reference :default "/Game/GameMode/Input/IA_Space.IA_Space"))
  (bind _returnvalue (Transformation|GetActorLocation))
  (bind _activespline (Variables|Default|GetActiveSpline))
  (bind _bisbook (Variables|Default|GetbIsBook))
  (bind _returnvalue_2 (Spline|FindLocationClosesttoWorldLocation _activespline _returnvalue "World"))
  (:Triggered
    (if (not _bisbook)
      (Pawn|Input|AddMovementInput (+ (Math|Vector|SelectVector (* (Math|Vector|Normalize (- _returnvalue_2 _returnvalue)) (Variables|Default|GetCorrection)) "0, 0, 0" (> (Math|Vector|Distance(Vector) _returnvalue _returnvalue_2) (Variables|Default|GetThreshold))) (Spline|FindDirectionClosesttoWorldLocation _activespline _returnvalue "World")) 1.0 false)))
  (:Started
    (if (not _bisbook)
      (bind _returnvalue_3 (Audio|CreateSound2D "/Game/Sfx/234_OutsideWalking.234_OutsideWalking" 16.0 1.0 0.0 0))
      (bind _output_get (Variables|Default|SetWalking _returnvalue_3))
      (Audio|Components|Audio|Play _output_get 1.2)))
  (:Canceled
    (bind _walking (Variables|Default|GetWalking :!label _label)
      (:then
        (Audio|Components|Audio|Stop _walking))
      (:else)))
  (:Completed
    (goto _label)))

(event Input|EnhancedActionEvents|EnhancedInputActionIA_Look
  (params (ActionValue :type Vector%202D%20Structure) (ElapsedSeconds :type Float%20%28double-precision%29) (TriggeredSeconds :type Float%20%28double-precision%29) (InputAction :type Input%20Action%20Object%20Reference :default "/Game/GameMode/Input/IA_Look.IA_Look"))
  (bind _returnvalue (Math|Float|MakeLiteralFloat 2.0))
  (bind _returnvalue_2 (* _returnvalue -1.0))
  (:Triggered
    (if (not (Variables|Default|GetbIsBook))
      (bind _output_get (Variables|Default|SetSmoothedVector (Math|Vector2D|MakeVector2D (Math|Float|Clamp(Float) (.x (Class|KismetMathLibrary|Vector2DInterpto (Variables|Default|GetSmoothedVector) (Math|Vector2D|MakeVector2D (.x ActionValue) (.y ActionValue)) (Utilities|Time|GetWorldDeltaSeconds) (Variables|Default|GetLookSmoothSpeed))) _returnvalue_2 _returnvalue) (Math|Float|Clamp(Float) (.y (Class|KismetMathLibrary|Vector2DInterpto (Variables|Default|GetSmoothedVector) (Math|Vector2D|MakeVector2D (.x ActionValue) (.y ActionValue)) (Utilities|Time|GetWorldDeltaSeconds) (Variables|Default|GetLookSmoothSpeed))) _returnvalue_2 _returnvalue))))
      (Pawn|Input|AddControllerYawInput (.x _output_get))
      (Pawn|Input|AddControllerPitchInput (.y _output_get))))
  (:Started
    (Variables|Default|SetbNotLooking false))
  (:Canceled
    (Variables|Default|SetbNotLooking true :!label _label))
  (:Completed
    (goto _label)))

(event EventBeginPlay
  (bind _returnvalue (Game|GetPlayerController 0))
  (bind _returnvalue_2 (Pawn|GetControlRotation _returnvalue :!class /Script/Engine.Controller))
  (Utilities|FlowControl|Sequence
    (:then_0
      (bind _closest (CallFunction|GetClosestSpline))
      (Variables|Default|SetActiveSpline _closest)
      (Actor|Tick|SetActorTickEnabled true)
      (Input|SetInputModeGameOnly (Game|GetPlayerController 0) true))
    (:then_1
      (bind _asbp_parting_game_instance (Utilities|Casting|CastToBP_PartingGameInstance (Game|GetGameInstance)))
      (bind _returnvalue_3 (Default|CreateSound _asbp_parting_game_instance "/Game/Music/2_DivergingPath.2_DivergingPath" 2.0 false))
      (bind _output_get (Variables|Default|SetMusic _returnvalue_3))
      (Audio|Components|Audio|FadeIn _output_get 4.0 1.0 0.0 "Linear" :!class /Script/Engine.AudioComponent)
      (bind _returnvalue_4 (Default|CreateSound _asbp_parting_game_instance "/Game/Sfx/2_DivergingPathAmbience.2_DivergingPathAmbience" 4.0 false))
      (bind _output_get_2 (Variables|Default|SetAmbiance _returnvalue_4))
      (Audio|Components|Audio|FadeIn _output_get_2 4.0 1.0 0.0 "Linear" :!class /Script/Engine.AudioComponent))
    (:then_2
      (Utilities|FlowControl|Delay 1.5)
      (bind _output_get_3 (Variables|Default|SetTemp (.pitch _returnvalue_2)))
      (bind _output_get_4 (Variables|Default|SetTemp2 (.yaw _returnvalue_2)))
      (bind _alpha (Timeline|Pan PlayFromStart)
        (:Update
          (Pawn|SetControlRotation (Game|GetPlayerController 0) (Math|Rotator|MakeRotator (.roll _returnvalue_2) (Math|Float|Lerp _output_get_3 -82.0 _alpha) (Math|Float|Lerp _output_get_4 -5e+01 _alpha))))
        (:Finished
          (if (Variables|Default|GetbTemp)
            (Variables|Default|SetbTemp false)
            (Timeline|Pan ReverseFromEnd)
            (else
              (Variables|Default|SetbIsBook false))))))))

(event EventTick
  (params (DeltaSeconds :type Float%20%28single-precision%29))
  (bind _returnvalue (Transformation|GetActorLocation))
  (bind _returnvalue_2 (Game|GetPlayerCameraManager 0))
  (bind _returnvalue_3 (Game|GetPlayerCameraManager 0))
  (bind _returnvalue_4 (Transformation|GetActorLocation))
  (bind _constrait (Variables|Default|GetConstrait))
  (bind _munin (Variables|Default|GetMunin))
  (bind _munin_2 (Variables|Default|GetMunin))
  (bind _playerspline (Variables|Default|GetPlayerSpline))
  (bind _munin_3 (Variables|Default|GetMunin))
  (bind _munin_4 (Variables|Default|GetMunin))
  (bind _figurespline (Variables|Default|GetFigureSpline))
  (bind _figurespline_2 (Variables|Default|GetFigureSpline))
  (bind _returnvalue_5 (Transformation|GetActorLocation _munin_3))
  (bind _returnvalue_6 (Transformation|GetActorLocation _munin_2))
  (bind _z (Math|Vector|BreakVector _returnvalue))
  (bind _spline (Variables|/Game/2_Scene1/BP_Spline.BP_Spline_C|GetSpline _playerspline))
  (bind _spline_2 (Variables|/Game/2_Scene1/BP_Spline.BP_Spline_C|GetSpline _figurespline))
  (bind _spline_3 (Variables|/Game/2_Scene1/BP_Spline.BP_Spline_C|GetSpline _figurespline_2))
  (bind _returnvalue_7 (Spline|FindLocationClosesttoWorldLocation _spline_3 (Math|Vector|MakeVector 127557.135571 -57362.404877 1447.631975) "World"))
  (bind _returnvalue_8 (Spline|FindLocationClosesttoWorldLocation _spline _returnvalue_4 "World"))
  (Utilities|FlowControl|Sequence
    (:then_0
      (if (Variables|Default|GetbIsMM)
        (if (not (Variables|Default|GetbIsBook))
          (Variables|/Script/Engine.PlayerCameraManager|SetViewYawMax _returnvalue_2 359.99)
          (Variables|/Script/Engine.PlayerCameraManager|SetViewYawMin _returnvalue_2 0.0)
          (Utilities|FlowControl|Sequence
            (:then_0
              (Utilities|FlowControl|Gate true :!label _label
                (:Exit
                  (Transformation|SetActorLocation _munin_2 (Math|Vector|MakeVector (.x (+ _returnvalue_6 (* (Spline|FindDirectionClosesttoWorldLocation _spline_2 _returnvalue_5 "World") (Variables|Default|GetSpeed) (Math|Float|SelectFloat (Math|Float|MapRangeClamped (- (Class|SplineComponent|GetDistanceAlongSplineatLocation _spline_2 (Transformation|GetActorLocation) "World") (Class|SplineComponent|GetDistanceAlongSplineatLocation _spline_2 _returnvalue_5 "World")) -5e+02 0.0 0.2 12.0) 1.0 (Variables|Default|GetFollow)) (Variables|Default|GetMuninSpeed)))) (.y (+ _returnvalue_6 (* (Spline|FindDirectionClosesttoWorldLocation _spline_2 _returnvalue_5 "World") (Variables|Default|GetSpeed) (Math|Float|SelectFloat (Math|Float|MapRangeClamped (- (Class|SplineComponent|GetDistanceAlongSplineatLocation _spline_2 (Transformation|GetActorLocation) "World") (Class|SplineComponent|GetDistanceAlongSplineatLocation _spline_2 _returnvalue_5 "World")) -5e+02 0.0 0.2 12.0) 1.0 (Variables|Default|GetFollow)) (Variables|Default|GetMuninSpeed)))) (.Z (Math|Vector|BreakVector _returnvalue_6))) false false)
                  (Utilities|FlowControl|Sequence
                    (:then_0
                      (if (> (Class|SplineComponent|GetDistanceAlongSplineatLocation (Variables|/Game/2_Scene1/BP_Spline.BP_Spline_C|GetSpline (Variables|Default|GetPlayerSpline)) (Transformation|GetActorLocation) "World") 6e+03)
                        (Utilities|FlowControl|DoOnce false
                          (:Completed
                            (bind _asbp_parting_game_instance (Utilities|Casting|CastToBP_PartingGameInstance (Game|GetGameInstance)))
                            (bind _returnvalue_9 (Default|CreateSound _asbp_parting_game_instance "/Game/Sfx/1_Swell.1_Swell" 1.0 false))
                            (Audio|Components|Audio|Play _returnvalue_9 0.0)
                            (Default|LoadLevel _asbp_parting_game_instance "/Game/3_Scene2/Scene2Old.Scene2Old" 1e+01)
                            (Utilities|FlowControl|Delay 2.0)
                            (Variables|Default|SetbIsBook true)))))
                    (:then_1
                      (if (Variables|Default|GetFollow)
                        (if (> (Class|SplineComponent|GetDistanceAlongSplineatLocation (Variables|/Game/2_Scene1/BP_Spline.BP_Spline_C|GetSpline (Variables|Default|GetFigureSpline)) _returnvalue "World") (Math|Random|RandomFloatinRange 4e+03 5e+03))
                          (Transformation|SetActorLocationAndRotation (Math|Vector|MakeVector 1.2476e+05 -5.717e+04 _z) "0, 0, 0")
                          (Transformation|SetActorLocation (Math|Vector|MakeVector (.x _returnvalue_8) (.y _returnvalue_8) _z) false false)
                          (Pawn|SetControlRotation (Game|GetPlayerController 0) (Math|Rotator|MakeRotator 0.0 0.0 0.0))
                          (Transformation|SetActorLocation _munin (Math|Vector|MakeVector (.x _returnvalue_7) (.y _returnvalue_7) (.z (Transformation|GetActorLocation _munin))) false false)
                          (Variables|Default|SetFollow false)
                          (Utilities|FlowControl|Sequence
                            (:then_0
                              (goto _label_2 Reset))
                            (:then_1
                              (goto _label Close))))))
                    (:then_2
                      (if (Utilities|Time|IsValidTimerHandle (Variables|Default|GetRotationTimerHandle))
                        _
                        (else
                          (CallFunction|RandomRotation)))
                      (Transformation|AddActorLocalRotation _munin_4 (Math|Rotator|MakeRotator 0.0 0.0 0.15) false false)
                      (Transformation|AddActorLocalOffset _munin_4 (Math|Vector|MakeVector 0.0 0.0 (* (Math|Trig|Sin(Radians) (* (Utilities|Time|GetTimeSeconds) 3.5)) 0.5)) false false))))))
            (:then_1
              (bind _transition (Variables|Default|GetTransition)
                (:then
                  (Variables|Default|SetActiveSpline (Variables|/Game/2_Scene1/BP_Spline.BP_Spline_C|GetSpline (select (or (< (- (.yaw (Transformation|GetActorRotation _transition)) (.yaw (Pawn|GetControlRotation :!class /Script/Engine.Pawn))) -2.3e+02) (and (< (- (.yaw (Transformation|GetActorRotation _transition)) (.yaw (Pawn|GetControlRotation :!class /Script/Engine.Pawn))) 84.0) (> (- (.yaw (Transformation|GetActorRotation _transition)) (.yaw (Pawn|GetControlRotation :!class /Script/Engine.Pawn))) -7e+01))) (Variables|/Game/2_Scene1/BP_SplineTransition.BP_SplineTransition_C|GetSplineRight _transition) (Variables|/Game/2_Scene1/BP_SplineTransition.BP_SplineTransition_C|GetSplineLeft _transition))))
                  (Utilities|FlowControl|DoOnce false :!label _label_2
                    (:Completed
                      (if (or (< (- (.yaw (Transformation|GetActorRotation _transition)) (.yaw (Pawn|GetControlRotation :!class /Script/Engine.Pawn))) -2.3e+02) (and (< (- (.yaw (Transformation|GetActorRotation _transition)) (.yaw (Pawn|GetControlRotation :!class /Script/Engine.Pawn))) 84.0) (> (- (.yaw (Transformation|GetActorRotation _transition)) (.yaw (Pawn|GetControlRotation :!class /Script/Engine.Pawn))) -7e+01)))
                        (Variables|Default|SetFollow true))
                      (CallFunction|Continue))))
                (:else)))))
        (else
          (Utilities|FlowControl|Sequence
            (:then_0
              (bind _transition_2 (Variables|Default|GetTransition)
                (:then
                  (if (== (select (or (< (- (.yaw (Transformation|GetActorRotation _transition_2)) (.yaw (Pawn|GetControlRotation :!class /Script/Engine.Pawn))) -2.7e+02) (and (< (- (.yaw (Transformation|GetActorRotation _transition_2)) (.yaw (Pawn|GetControlRotation :!class /Script/Engine.Pawn))) 1e+02) (> (- (.yaw (Transformation|GetActorRotation _transition_2)) (.yaw (Pawn|GetControlRotation :!class /Script/Engine.Pawn))) 2e+01))) (Variables|/Game/2_Scene1/BP_SplineTransition.BP_SplineTransition_C|GetSplineRight _transition_2) (Variables|/Game/2_Scene1/BP_SplineTransition.BP_SplineTransition_C|GetSplineLeft _transition_2)) (Variables|Default|GetActiveSpline))
                    (if (not (stale _output_get)) :!label _label_3
                      (Variables|/Script/Engine.PlayerCameraManager|SetViewYawMax _returnvalue_3 (+ (.yaw (Math|Rotator|MakeRotfromX (Spline|FindDirectionClosesttoWorldLocation (Variables|Default|GetActiveSpline) (Transformation|GetActorLocation) "World"))) _constrait))
                      (Variables|/Script/Engine.PlayerCameraManager|SetViewYawMin _returnvalue_3 (- (.yaw (Math|Rotator|MakeRotfromX (Spline|FindDirectionClosesttoWorldLocation (Variables|Default|GetActiveSpline) (Transformation|GetActorLocation) "World"))) _constrait)))
                    (else
                      (bind _output_get (Variables|Default|SetbInTransition true))
                      (CallFunction|TransitionSplines (Variables|Default|GetActiveSpline) (Variables|/Game/2_Scene1/BP_Spline.BP_Spline_C|GetSpline (select (or (< (- (.yaw (Transformation|GetActorRotation _transition_2)) (.yaw (Pawn|GetControlRotation :!class /Script/Engine.Pawn))) -2.7e+02) (and (< (- (.yaw (Transformation|GetActorRotation _transition_2)) (.yaw (Pawn|GetControlRotation :!class /Script/Engine.Pawn))) 1e+02) (> (- (.yaw (Transformation|GetActorRotation _transition_2)) (.yaw (Pawn|GetControlRotation :!class /Script/Engine.Pawn))) 2e+01))) (Variables|/Game/2_Scene1/BP_SplineTransition.BP_SplineTransition_C|GetSplineRight _transition_2) (Variables|/Game/2_Scene1/BP_SplineTransition.BP_SplineTransition_C|GetSplineLeft _transition_2))))
                      (Variables|Default|SetActiveSpline (Variables|/Game/2_Scene1/BP_Spline.BP_Spline_C|GetSpline (select (or (< (- (.yaw (Transformation|GetActorRotation _transition_2)) (.yaw (Pawn|GetControlRotation :!class /Script/Engine.Pawn))) -2.7e+02) (and (< (- (.yaw (Transformation|GetActorRotation _transition_2)) (.yaw (Pawn|GetControlRotation :!class /Script/Engine.Pawn))) 1e+02) (> (- (.yaw (Transformation|GetActorRotation _transition_2)) (.yaw (Pawn|GetControlRotation :!class /Script/Engine.Pawn))) 2e+01))) (Variables|/Game/2_Scene1/BP_SplineTransition.BP_SplineTransition_C|GetSplineRight _transition_2) (Variables|/Game/2_Scene1/BP_SplineTransition.BP_SplineTransition_C|GetSplineLeft _transition_2)))))))
                (:else
                  (goto _label_3))))))))
    (:then_1
      (if (not (Variables|Default|GetbIsBook))
        (CallFunction|SmoothLook)))))

(fn ConstructionScript)

(fn HasTag
  (params (Component :type Actor%20Component%20Object%20Reference) (Tag :type Name))
  (for _array_element (Variables|/Script/Engine.ActorComponent|GetComponentTags Component)
    (if (== _array_element Tag)
      (return true)))
  (return false))

(fn GetClosestSpline
  (bind _returnvalue (Transformation|GetActorLocation))
  (bind _outactors (Actor|GetAllActorsOfClass "/Game/2_Scene1/BP_Spline.BP_Spline_C"))
  (for _array_element _outactors
    (if (< (Class|KismetMathLibrary|VectorDistanceSquared (Spline|FindLocationClosesttoWorldLocation (Variables|/Game/2_Scene1/BP_Spline.BP_Spline_C|GetSpline _array_element) _returnvalue "World") _returnvalue) (LocalVariables|GetMin))
      (LocalVariables|SetMin (Class|KismetMathLibrary|VectorDistanceSquared (Spline|FindLocationClosesttoWorldLocation (Variables|/Game/2_Scene1/BP_Spline.BP_Spline_C|GetSpline _array_element) _returnvalue "World") _returnvalue))
      (LocalVariables|SetSpline (Variables|/Game/2_Scene1/BP_Spline.BP_Spline_C|GetSpline _array_element))))
  (return (LocalVariables|GetSpline) (LocalVariables|GetMin)))