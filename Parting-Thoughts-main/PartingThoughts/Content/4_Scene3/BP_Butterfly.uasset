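; Scene 3 butterfly that carries a ticket, hopping along a chain of splines and landing points relative to the player.
; Each Walk call triggers a timeline flight burst, scaled by player distance, with random wobble and correction back to the spline.
; At spline start it lands, enlarging the ticket at two stops, then departs for the next spline once the player's spline distance leads enough.
; Randomized timelines flap the wings.
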(event Custom|Walk
  (bind _returnvalue (Transformation|GetActorLocation))
  (bind _returnvalue_2 (Transformation|GetActorLocation))
  (bind _player (Variables|Default|GetPlayer))
  (bind _ticket (Variables|Default|GetTicket))
  (bind _ticket_2 (Variables|Default|GetTicket))
  (bind _originalscale (Variables|Default|GetOriginalScale))
  (if (not (Variables|Default|GetbDeparting))
    (if (Variables|Default|GetbShouldFly)
      (Utilities|FlowControl|Sequence
        (:then_0
          (Audio|Components|Audio|Stop (Variables|Default|GetFlyCorrect)))
        (:then_1
          (Transformation|SetRelativeScale3D _ticket (Variables|Default|GetOriginalScale))
          (Transformation|SetRelativeRotation _ticket (Variables|Default|GetOriginalRotation) false false)
          (Components|Timeline|SetPlayRate (Variables|Default|GetFly) (/ 1.0 0.5))
          (Variables|Default|SetFlapFactor 1.0)
          (bind _output_get (Variables|Default|SetFactor (Math|Float|MapRangeClamped (- (Class|SplineComponent|GetDistanceAlongSplineatLocation (Variables|/Game/4_Scene3/BP_PlayerScene3.BP_PlayerScene3_C|GetActiveSpline _player) (Spline|FindLocationClosesttoWorldLocation (Variables|/Game/4_Scene3/BP_PlayerScene3.BP_PlayerScene3_C|GetActiveSpline _player) (Transformation|GetActorLocation _player) "Local") "Local") (Class|SplineComponent|GetDistanceAlongSplineatLocation (Variables|/Game/4_Scene3/BP_PlayerScene3.BP_PlayerScene3_C|GetActiveSpline _player) (Spline|FindLocationClosesttoWorldLocation (Variables|/Game/4_Scene3/BP_PlayerScene3.BP_PlayerScene3_C|GetActiveSpline _player) (Transformation|GetActorLocation) "Local") "Local")) -5e+02 4e+02 0.9 2.5)))
          (CallFunction|MakeOffset)
          (bind _alpha (Timeline|Fly PlayFromStart)
            (:Update
              (Transformation|SetActorLocationAndRotation (+ _returnvalue (* 21.0 (Spline|FindDirectionClosesttoWorldLocation (Variables|Default|GetActiveSpline) _returnvalue "World") -1.0 _alpha _output_get) (Variables|Default|GetOffset)) (Math|Rotator|MakeRotfromX (Spline|FindDirectionClosesttoWorldLocation (Variables|Default|GetActiveSpline) _returnvalue "World")))
              (if (< (Math|Vector|Distance(Vector) (Spline|GetLocationatSplinePoint (Variables|Default|GetActiveSpline) 0 "World") (Spline|FindLocationClosesttoWorldLocation (Variables|Default|GetActiveSpline) (Transformation|GetActorLocation) "World")) 1e+01) :!label _label
                (Audio|Components|Audio|Stop (Variables|Default|GetFly))
                (Utilities|FlowControl|Sequence
                  (:then_0
                    (Variables|Default|SetbShouldFly false)
                    (Utilities|Time|ClearandInvalidateTimerbyHandle (Variables|Default|GetTimer))
                    (Rendering|Material|SetScalarParameterValue "/Game/4_Scene3/MPC_Toggle.MPC_Toggle" "Toggle" 1.0 :!class /Script/Engine.KismetMaterialLibrary))
                  (:then_1
                    (Components|Timeline|SetPlayRate (Variables|Default|GetLand) 0.5)
                    (bind _output_get_2 (Variables|Default|SetStartLoc (Transformation|GetActorLocation)))
                    (bind _output_get_3 (Variables|Default|SetStartRot (Transformation|GetActorRotation)))
                    (bind _output_get_4 (Variables|Default|SetTemp (Components|Animation|GetPlayRate (Variables|Default|GetWings))))
                    (bind _alpha_2 (Timeline|Land PlayFromStart)
                      (:Update
                        (Transformation|SetActorLocationAndRotation (Math|Vector|Lerp(Vector) _output_get_2 (Utilities|Array|Get(acopy) (Variables|Default|GetLocations) (Variables|Default|GetIndex)) _alpha_2) (Math|Rotator|Lerp(Rotator) _output_get_3 (Math|Rotator|FindLookatRotation (Math|Vector|MakeVector (.X (Math|Vector|BreakVector (Utilities|Array|Get(acopy) (Variables|Default|GetLocations) (Variables|Default|GetIndex)))) (.Y (Math|Vector|BreakVector (Utilities|Array|Get(acopy) (Variables|Default|GetLocations) (Variables|Default|GetIndex)))) 0.0) (Math|Vector|MakeVector (.X (Math|Vector|BreakVector _output_get_2)) (.Y (Math|Vector|BreakVector _output_get_2)) 0.0)) _alpha_2))
                        (Components|Timeline|SetPlayRate (Variables|Default|GetWings) (Math|Float|Lerp _output_get_4 0.0 _alpha_2)))
                      (:Finished
                        (Components|Activation|Deactivate (Variables|Default|GetNS_Trail))
                        (if (or (== (Variables|Default|GetIndex) 2) (== (Variables|Default|GetIndex) 4))
                          (Collision|SetCollisionEnabled (Variables|Default|GetCollision) "QueryOnly")
                          (Utilities|FlowControl|Delay 2.0)
                          (Components|Timeline|SetPlayRate (Variables|Default|GetTicketScale) 1.0)
                          (bind _alpha_3 (Timeline|TicketScale PlayFromStart)
                            (:Update
                              (Transformation|SetRelativeScale3D _ticket_2 (Math|Vector|Lerp(Vector) _originalscale (* _originalscale 2.5) _alpha_3))
                              (Transformation|SetRelativeRotation _ticket_2 (Math|Rotator|Lerp(Rotator) (Variables|Default|GetOriginalRotation) "-48.000000,-4.000000,51.000000" _alpha_3 true) false false))))))))))
            (:Finished
              (Utilities|Time|ClearandInvalidateTimerbyHandle (Variables|Default|GetTimer))
              (bind _output_get_5 (Variables|Default|SetEndLoc (Spline|FindLocationClosesttoWorldLocation (Variables|Default|GetActiveSpline) _returnvalue_2 "World")))
              (Components|Timeline|SetPlayRate (Variables|Default|GetFlyCorrect) (/ 1.0 0.16))
              (Timeline|FlyCorrect PlayFromStart
                (:Update
                  (Transformation|SetActorLocation (Math|Interpolation|VInterpTo _returnvalue_2 _output_get_5 (Utilities|Time|GetWorldDeltaSeconds) 3.0) false false)
                  (goto _label))
                (:Finished
                  (Variables|Default|SetFlapFactor 0.3)))))))
      (elif (> (- (Class|SplineComponent|GetDistanceAlongSplineatLocation (Variables|/Game/4_Scene3/BP_PlayerScene3.BP_PlayerScene3_C|GetActiveSpline _player) (Spline|FindLocationClosesttoWorldLocation (Variables|/Game/4_Scene3/BP_PlayerScene3.BP_PlayerScene3_C|GetActiveSpline _player) (Transformation|GetActorLocation _player) "Local") "Local") (Class|SplineComponent|GetDistanceAlongSplineatLocation (Variables|/Game/4_Scene3/BP_PlayerScene3.BP_PlayerScene3_C|GetActiveSpline _player) (Spline|FindLocationClosesttoWorldLocation (Variables|/Game/4_Scene3/BP_PlayerScene3.BP_PlayerScene3_C|GetActiveSpline _player) (Transformation|GetActorLocation) "Local") "Local")) 1.5e+02)
        (Utilities|FlowControl|Sequence
          (:then_0
            (Variables|Default|SetbDeparting true)
            (Audio|Components|Audio|Stop (Variables|Default|GetLand))
            (bind _output_get_6 (Variables|Default|SetIndex (Math|Integer|%(Integer) (+ (Variables|Default|GetIndex) 1) (Utilities|Array|Length (Variables|Default|GetSplines)))))
            (Rendering|Material|SetScalarParameterValue "/Game/4_Scene3/MPC_Toggle.MPC_Toggle" "Toggle" (Math|Conversions|ToFloat(Boolean) (or (== _output_get_6 2) (== _output_get_6 4))) :!class /Script/Engine.KismetMaterialLibrary)
            (bind _output_get_7 (Variables|Default|SetActiveSpline (Variables|/Game/2_Scene1/BP_Spline.BP_Spline_C|GetSpline (Utilities|Array|Get(acopy) (Variables|Default|GetSplines) _output_get_6))))
            (Components|Activation|Activate (Variables|Default|GetNS_Trail) false))
          (:then_1
            (bind _output_get_8 (Variables|Default|SetStartLoc (Transformation|GetActorLocation)))
            (bind _output_get_9 (Variables|Default|SetStartRot (Transformation|GetActorRotation)))
            (bind _alpha_4 (Timeline|Depart PlayFromStart)
              (:Update
                (Transformation|SetActorLocationAndRotation (Math|Vector|Lerp(Vector) _output_get_8 (Spline|GetLocationatSplinePoint _output_get_7 (Utilities|Operators|Subtract (Spline|GetNumberOfSplinePoints _output_get_7) 1) "World") _alpha_4) (Math|Rotator|Lerp(Rotator) _output_get_9 (Math|Rotator|FindLookatRotation (Math|Vector|MakeVector (.X (Math|Vector|BreakVector (Spline|GetLocationatSplinePoint _output_get_7 (Utilities|Operators|Subtract (Spline|GetNumberOfSplinePoints _output_get_7) 1) "World"))) (.Y (Math|Vector|BreakVector (Spline|GetLocationatSplinePoint _output_get_7 (Utilities|Operators|Subtract (Spline|GetNumberOfSplinePoints _output_get_7) 1) "World"))) 0.0) (Math|Vector|MakeVector (.X (Math|Vector|BreakVector _output_get_8)) (.Y (Math|Vector|BreakVector _output_get_8)) 0.0)) _alpha_4))
                (Components|Timeline|SetPlayRate (Variables|Default|GetWings) (Math|Float|Lerp 2.0 1.0 _alpha_4)))
              (:Finished
                (Variables|Default|SetbDeparting false)
                (Variables|Default|SetbShouldFly true)
                (Collision|SetCollisionEnabled (Variables|Default|GetCollision) "NoCollision")
                (Variables|Default|SetFlapFactor 0.3)))))))))

(event Custom|MakeOffset
  (Variables|Default|SetOffset (* (Math|Random|RandomUnitVector) (Math|Random|RandomFloatinRange 2.0 4.0)))
  (bind _output_get (Variables|Default|SetOffsetTime (Math|Random|RandomFloatinRange 0.1 0.3)))
  (bind _returnvalue (Utilities|Time|SetTimerbyEvent (delegate Custom|MakeOffset) _output_get))
  (Variables|Default|SetTimer _returnvalue)
  (CallFunction|Flap))

(event Custom|Flap
  (bind _returnvalue (Math|Random|RandomFloatinRange 2.0 4.0))
  (bind _wings (Variables|Default|GetWings))
  (bind _flapfactor (Variables|Default|GetFlapFactor))
  (bind _returnvalue_2 (* _returnvalue _flapfactor))
  (Utilities|FlowControl|Sequence
    (:then_0
      (Components|Timeline|SetPlayRate _wings _returnvalue_2)
      (bind _output_get (Variables|Default|SetLower (Math|Random|RandomFloatinRange -6e+01 -1e+01)))
      (bind _output_get_2 (Variables|Default|SetUpper (Math|Random|RandomFloatinRange 5e+01 85.0)))
      (bind _alpha (Timeline|Wings Play)
        (:Update
          (Transformation|SetRelativeRotation (Variables|Default|GetLeft) (Math|Rotator|MakeRotator (Math|Float|Lerp _output_get _output_get_2 (- 1.0 _alpha)) 0.0 0.0) false false)
          (Transformation|SetRelativeRotation (Variables|Default|GetRight) (Math|Rotator|MakeRotator (* (Math|Float|Lerp _output_get _output_get_2 (- 1.0 _alpha)) -1.0) 0.0 0.0) false false))
        (:Finished
          (Components|Timeline|SetPlayRate _wings (Math|Float|SelectFloat _returnvalue_2 (Components|Animation|GetPlayRate _wings) (Variables|Default|GetbShouldFly)))
          (Timeline|Wings PlayFromStart))))
    (:then_1
      (Utilities|Time|SetTimerbyEvent (delegate Custom|NewFlap) (Variables|Default|GetOffsetTime)))))

(event Custom|NewFlap
  (bind _returnvalue (Math|Random|RandomFloatinRange 2.0 4.0))
  (bind _wings (Variables|Default|GetWings))
  (bind _flapfactor (Variables|Default|GetFlapFactor))
  (bind _returnvalue_2 (* _returnvalue _flapfactor))
  (Components|Timeline|SetPlayRate _wings _returnvalue_2)
  (bind _output_get (Variables|Default|SetLower (Math|Random|RandomFloatinRange -6e+01 -1e+01)))
  (bind _output_get_2 (Variables|Default|SetUpper (Math|Random|RandomFloatinRange 5e+01 85.0)))
  (bind _alpha (Timeline|Wings Play)
    (:Update
      (Transformation|SetRelativeRotation (Variables|Default|GetLeft) (Math|Rotator|MakeRotator (Math|Float|Lerp _output_get _output_get_2 (- 1.0 _alpha)) 0.0 0.0) false false)
      (Transformation|SetRelativeRotation (Variables|Default|GetRight) (Math|Rotator|MakeRotator (* (Math|Float|Lerp _output_get _output_get_2 (- 1.0 _alpha)) -1.0) 0.0 0.0) false false))
    (:Finished
      (Components|Timeline|SetPlayRate _wings (Math|Float|SelectFloat _returnvalue_2 (Components|Animation|GetPlayRate _wings) (Variables|Default|GetbShouldFly)))
      (Timeline|Wings PlayFromStart))))

(event Custom|Highlight
  (params (bHighlight :type Boolean))
  (Rendering|SetRenderCustomDepth (Variables|Default|GetTicket) bHighlight))

(event EventBeginPlay
  (bind _ticket (Variables|Default|GetTicket))
  (Utilities|FlowControl|Sequence
    (:then_0
      (bind _returnvalue (Actor|GetActorOfClass "/Game/4_Scene3/BP_PlayerScene3.BP_PlayerScene3_C"))
      (Variables|Default|SetPlayer _returnvalue)
      (bind _output_get (Variables|Default|SetActiveSpline (Variables|/Game/2_Scene1/BP_Spline.BP_Spline_C|GetSpline (Utilities|Array|Get(acopy) (Variables|Default|GetSplines)))))
      (Transformation|SetActorLocationAndRotation (Spline|GetLocationatSplinePoint _output_get 3 "World") (Math|Rotator|MakeRotfromX (Class|SplineComponent|GetDirectionatSplinePoint _output_get 3 "World")))
      (for _array_element (Variables|Default|GetLandings)
        (Utilities|Array|Add (Variables|Default|GetLocations) (Transformation|GetActorLocation _array_element))))
    (:then_1
      (CallFunction|Flap)
      (Variables|Default|SetOriginalScale (Variables|/Script/Engine.SceneComponent|GetRelativeScale3D _ticket))
      (Variables|Default|SetOriginalRotation (Variables|/Script/Engine.SceneComponent|GetRelativeRotation _ticket)))))

(fn ConstructionScript)