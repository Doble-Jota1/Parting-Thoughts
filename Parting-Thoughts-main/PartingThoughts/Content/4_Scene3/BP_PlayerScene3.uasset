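; First-person player for Scene 3, which chases a butterfly along a BP_Path spline and can click to open TrainStationLast.
; Space runs a timeline that moves the player toward the next path point and triggers the butterfly's walk; the upcoming point gets a highlight material.
; A per-tick camera trace toggles the butterfly's highlight and enables the level-changing click.
; Look input is interpolated and clamped, then eases out after release.
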(event Input|EnhancedActionEvents|EnhancedInputActionIA_Look
  (params (ActionValue :type Vector%202D%20Structure) (ElapsedSeconds :type Float%20%28double-precision%29) (TriggeredSeconds :type Float%20%28double-precision%29) (InputAction :type Input%20Action%20Object%20Reference :default "/Game/GameMode/Input/IA_Look.IA_Look"))
  (bind _returnvalue (Math|Float|MakeLiteralFloat 2.0))
  (bind _returnvalue_2 (* _returnvalue -1.0))
  (:Triggered
    (bind _output_get (Variables|Default|SetSmoothedVector (Math|Vector2D|MakeVector2D (Math|Float|Clamp(Float) (.x (Class|KismetMathLibrary|Vector2DInterpto (Variables|Default|GetSmoothedVector) (Math|Vector2D|MakeVector2D (.x ActionValue) (.y ActionValue)) (Utilities|Time|GetWorldDeltaSeconds) (Variables|Default|GetLookSmoothSpeed))) _returnvalue_2 _returnvalue) (Math|Float|Clamp(Float) (.y (Class|KismetMathLibrary|Vector2DInterpto (Variables|Default|GetSmoothedVector) (Math|Vector2D|MakeVector2D (.x ActionValue) (.y ActionValue)) (Utilities|Time|GetWorldDeltaSeconds) (Variables|Default|GetLookSmoothSpeed))) _returnvalue_2 _returnvalue))))
    (Pawn|Input|AddControllerYawInput (.x _output_get))
    (Pawn|Input|AddControllerPitchInput (.y _output_get)))
  (:Started
    (Variables|Default|SetbNotLooking false))
  (:Canceled
    (Variables|Default|SetbNotLooking true :!label _label))
  (:Completed
    (goto _label)))

(event Input|EnhancedActionEvents|EnhancedInputActionIA_Space
  (params (ActionValue :type Boolean) (ElapsedSeconds :type Float%20%28double-precision%29) (TriggeredSeconds :type Float%20%28double-precision%29) (InputAction :type Input%20Action%20Object%20Reference :default "/Game/GameMode/Input/IA_Space.IA_Space"))
  (bind _returnvalue (Transformation|GetActorLocation))
  (bind _paths (Variables|Default|GetPaths))
  (bind _paths_2 (Variables|Default|GetPaths))
  (bind _activespline (Variables|Default|GetActiveSpline))
  (bind _returnvalue_2 (Utilities|Array|Length _paths))
  (:Completed
    (if (not (Variables|Default|GetbIsBook))
      (Utilities|FlowControl|Sequence
        (:then_0
          (Audio|CreateSound2D "/Game/Sfx/234_OutsideWalking.234_OutsideWalking" 16.0 1.0 0.0 0))
        (:then_1
          (Variables|Default|SetbIsBook true)
          (Components|Timeline|SetPlayRate (Variables|Default|GetWalk) 1.5)
          (bind _output_get (Variables|Default|SetFactor (Math|Vector|Distance(Vector) (Transformation|GetWorldLocation (Utilities|Array|Get(acopy) _paths_2 (Variables|Default|GetIndex))) (Transformation|GetWorldLocation (Utilities|Array|Get(acopy) _paths_2 (Math|Integer|%(Integer) (+ (Variables|Default|GetIndex) 1) (Utilities|Array|Length _paths_2)))))))
          (bind _alpha (Timeline|Walk PlayFromStart)
            (:Update
              (Transformation|AddActorWorldOffset (* (Spline|GetDirectionatDistanceAlongSpline _activespline (Class|SplineComponent|GetDistanceAlongSplineatLocation _activespline _returnvalue "World") "World") _output_get 0.01 3.5 _alpha))
              (if (< (Math|Vector|Distance2D(Vector) _returnvalue (Transformation|GetWorldLocation (Utilities|Array|Get(acopy) _paths_2 (Math|Integer|%(Integer) (+ (Variables|Default|GetIndex) 1) (Utilities|Array|Length _paths_2))))) 1e+01)
                (Variables|Default|SetbIsBook false)
                (Utilities|FlowControl|Sequence
                  (:then_0
                    (Timeline|Walk Stop))
                  (:then_1
                    (Variables|Default|SetbIsBook false :!label _label)
                    (bind _output_get_2 (Variables|Default|SetIndex (Math|Integer|%(Integer) (+ (Variables|Default|GetIndex) 1) _returnvalue_2)))
                    (Rendering|Material|SetMaterial (Utilities|Array|Get(acopy) _paths (Variables|Default|GetIndex)) 0 (Variables|Default|GetPrevMaterial))
                    (Variables|Default|SetPrevMaterial (Rendering|Material|GetMaterial (Utilities|Array|Get(acopy) _paths (Math|Integer|%(Integer) (+ _output_get_2 1) _returnvalue_2)) 0))
                    (Rendering|Material|SetMaterial (Utilities|Array|Get(acopy) _paths (Math|Integer|%(Integer) (+ _output_get_2 1) _returnvalue_2)) 0 "/Game/4_Scene3/M_Highlight.M_Highlight")))))
            (:Finished
              (goto _label))))
        (:then_2
          (Default|Walk (Variables|Default|GetButterfly)))))))

(event Input|EnhancedActionEvents|EnhancedInputActionIA_LeftClick
  (params (ActionValue :type Boolean) (ElapsedSeconds :type Float%20%28double-precision%29) (TriggeredSeconds :type Float%20%28double-precision%29) (InputAction :type Input%20Action%20Object%20Reference :default "/Game/GameMode/Input/IA_LeftClick.IA_LeftClick"))
  (:Completed
    (Variables|Default|GetHit%20Component
      (:then
        (Actor|Tick|SetActorTickEnabled false)
        (Game|OpenLevel(byObjectReference) "/Game/5_Scene_Last/TrainStationLast.TrainStationLast"))
      (:else))))

(event EventBeginPlay
  (bind _index (Variables|Default|GetIndex))
  (Utilities|FlowControl|Sequence
    (:then_0
      (bind _returnvalue (Audio|CreateSound2D "/Game/Music/4_ChasingButterfly.4_ChasingButterfly" 1.0 1.0 0.0 0))
      (bind _output_get (Variables|Default|SetMUsic _returnvalue))
      (Audio|Components|Audio|Play _output_get 0.0)
      (Input|SetInputModeGameOnly (Game|GetPlayerController 0) true))
    (:then_1
      (bind _returnvalue_2 (Actor|GetActorOfClass "/Game/4_Scene3/BP_Path.BP_Path_C"))
      (Variables|Default|SetActiveSpline (Variables|/Game/4_Scene3/BP_Path.BP_Path_C|GetSpline _returnvalue_2))
      (bind _output_get_2 (Variables|Default|SetPaths (Variables|/Game/4_Scene3/BP_Path.BP_Path_C|GetPaths _returnvalue_2)))
      (Variables|Default|SetPrevMaterial (Rendering|Material|GetMaterial (Utilities|Array|Get(acopy) _output_get_2 (+ _index 1)) 0))
      (Rendering|Material|SetMaterial (Utilities|Array|Get(acopy) _output_get_2 (+ _index 1)) 0 "/Game/4_Scene3/M_Highlight.M_Highlight")
      (Transformation|SetActorLocation (Math|Vector|MakeVector (.x (Transformation|GetWorldLocation (Utilities|Array|Get(acopy) _output_get_2 _index))) (.y (Transformation|GetWorldLocation (Utilities|Array|Get(acopy) _output_get_2 _index))) (.z (Transformation|GetActorLocation))) false false))
    (:then_2
      (bind _returnvalue_3 (Actor|GetActorOfClass "/Game/4_Scene3/BP_Butterfly.BP_Butterfly_C"))
      (Variables|Default|SetButterfly _returnvalue_3))))

(event EventTick
  (params (DeltaSeconds :type Float%20%28single-precision%29))
  (bind _firstpersoncamera (Variables|Default|GetFirstPersonCamera))
  (bind _butterfly (Variables|Default|GetButterfly))
  (bind _returnvalue (Transformation|GetWorldLocation _firstpersoncamera))
  (Utilities|FlowControl|Sequence
    (:then_0
      (bind _outhit (Collision|LineTraceForObjects _returnvalue (+ _returnvalue (* (Math|Vector|GetForwardVector _firstpersoncamera) 2e+03)) (Utilities|Array|MakeArray "ObjectTypeQuery7") true 0 "None"))
      (if (not (== (Variables|Default|GetHit%20Component) (.HitComponent (Collision|BreakHitResult _outhit))))
        (Utilities|IsValid (.HitComponent (Collision|BreakHitResult _outhit))
          (:Is%20Valid
            (Default|Highlight _butterfly true))
          (:Is%20Not%20Valid
            _))
        (Variables|Default|GetHit%20Component
          (:then
            (Default|Highlight _butterfly false))
          (:else
            _))
        (Variables|Default|SetHit%20Component (.HitComponent (Collision|BreakHitResult _outhit)))))
    (:then_1
      (if (Variables|Default|GetbNotLooking)
        (bind _output_get (Variables|Default|SetSmoothedVector (Math|Vector2D|MakeVector2D (.x (Class|KismetMathLibrary|Vector2DInterpto (Variables|Default|GetSmoothedVector) (Math|Vector2D|MakeVector2D 0.0 0.0) (Utilities|Time|GetWorldDeltaSeconds) (Variables|Default|GetLookSmoothSpeed))) (.y (Class|KismetMathLibrary|Vector2DInterpto (Variables|Default|GetSmoothedVector) (Math|Vector2D|MakeVector2D 0.0 0.0) (Utilities|Time|GetWorldDeltaSeconds) (Variables|Default|GetLookSmoothSpeed))))))
        (Pawn|Input|AddControllerYawInput (.x _output_get))
        (Pawn|Input|AddControllerPitchInput (.y _output_get))))))

(fn ConstructionScript)

(fn HasTag
  (params (Component :type Actor%20Component%20Object%20Reference) (Tag :type Name))
  (for _array_element (Variables|/Script/Engine.ActorComponent|GetComponentTags Component)
    (if (== _array_element Tag)
      (return true)))
  (return false))