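; Game instance that handles level transitions with a white camera fade and matching audio fade-out.
; LoadLevel fades to white, opens the target level after the fade, then fades back in, using a default duration when given zero.
; In parallel it clears the tracked audio list and fades those sounds out over a longer time.
; CreateSound creates 2D sounds and registers them for that fade when flagged.
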(event Custom|FadeIn
  (params (Duration :type Float%20%28single-precision%29))
  (CameraFades|StartCameraFade (Game|GetPlayerCameraManager 0) 1.0 0.0 Duration "(R=1.000000,G=1.000000,B=1.000000,A=1.000000)" false true))

(event Custom|LoadLevel
  (params (Level :type World%20Soft%20Object%20Reference) (Duration :type Float%20%28single-precision%29))
  (bind _returnvalue (== Duration 0.0))
  (bind _audios (Variables|Default|GetAudios))
  (bind _returnvalue_2 (Math|Float|SelectFloat 2.0 Duration _returnvalue))
  (Utilities|FlowControl|Sequence
    (:then_0
      (CallFunction|FadeOut _returnvalue_2)
      (Utilities|FlowControl|Delay _returnvalue_2)
      (Game|OpenLevel(byObjectReference) Level)
      (Utilities|FlowControl|Delay 0.01)
      (CallFunction|Fadein 3.0))
    (:then_1
      (bind _output_get (Variables|Default|SetAudioTemp _audios))
      (Utilities|Array|Clear _audios)
      (for _array_element _output_get
        (Audio|Components|Audio|FadeOut _array_element (* _returnvalue_2 1.5) 0.0 "Linear" :!class /Script/Engine.AudioComponent)))))

(event Custom|FadeOut
  (params (Duration :type Float%20%28single-precision%29))
  (CameraFades|StartCameraFade (Game|GetPlayerCameraManager 0) 0.0 1.0 Duration "(R=1.000000,G=1.000000,B=1.000000,A=1.000000)" false true))

(fn CreateSound
  (params (Sound :type Sound%20Base%20Object%20Reference) (VolumeMultiplier :type Float%20%28single-precision%29) (bFade :type Boolean))
  (bind _returnvalue (Audio|CreateSound2D Sound VolumeMultiplier 1.0 0.0 0 true))
  (if bFade
    (Utilities|Array|Add (Variables|Default|GetAudios) _returnvalue))
  (return _returnvalue))