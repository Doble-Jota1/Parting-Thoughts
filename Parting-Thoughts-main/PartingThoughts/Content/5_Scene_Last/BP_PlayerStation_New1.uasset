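; Player pawn for the final train-station scene, opening with title cards and audio and ending in a farewell sequence that quits the game.
; Holding Space walks it along BP_Spline with smoothed look input; nearing the destination triggers Parting's fade, cards and end splash.
; Events raise the arm, present an attached book by timeline, and mouse-trace to reveal hovered components.
; Left-click is empty; the ticket-selection logic is disconnected.
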(event Custom|ShowBook
  (bind _returnvalue (Transformation|GetActorForwardVector))
  (bind _sphere (Variables|Default|GetSphere))
  (bind _returnvalue_2 (Transformation|GetWorldTransform _sphere))
  (bind _returnvalue_3 (* _returnvalue 1e+02))
  (bind _returnvalue_4 (- (.location _returnvalue_2) "0.000000,0.000000,100.000000"))
  (bind _returnvalue_5 (- _returnvalue_4 _returnvalue_3))
  (Variables|Default|SetbIsBook true)
  (bind _returnvalue_6 (Game|SpawnActorfromClass "/Game/1_TrainStation/BP_Book.BP_Book_C" (Math|Transform|MakeTransform _returnvalue_5 "0, 0, 0" "0.060000,0.060000,0.060000") "AlwaysSpawn" "MultiplyWithRoot" 0 0))
  (bind _output_get (Variables|Default|SetBook _returnvalue_6))
  (Transformation|AttachComponentToComponent _output_get (Variables|Default|GetSphere) "None" "KeepWorld" "KeepRelative" "KeepWorld" true)
  (bind _alpha (Timeline|BookTakeOut PlayFromStart)
    (:Update
      (Transformation|SetActorLocation (Variables|Default|GetBook) (Math|Vector|Lerp(Vector) _returnvalue_5 (.location _returnvalue_2) _alpha) false false))
    (:Finished
      (Utilities|FlowControl|Sequence
        (:then_0
          (Utilities|FlowControl|Delay 3.2)
          (Variables|Default|SetbBookTrace true)
          (Variables|/Script/Engine.PlayerController|SetbShowMouseCursor (Game|GetPlayerController 0) true))
        (:then_1
          (Utilities|FlowControl|Delay 1.0)
          (Default|StartShake (Variables|Default|GetBook)))))))

(event Custom|BookTrace
  (bind _returnvalue (Game|GetPlayerController 0))
  (bind (_worldlocation _worlddirection) (Game|Player|ConvertMouseLocationToWorldSpace _returnvalue))
  (bind _outhit (Collision|LineTraceForObjects _worldlocation (+ _worldlocation (* _worlddirection 5e+02)) (Utilities|Array|MakeArray "ObjectTypeQuery8") true 0 "None"))
  (if (not (== (Variables|Default|GetHit%20Component) (.HitComponent (Collision|BreakHitResult _outhit))))
    (Utilities|IsValid (.HitComponent (Collision|BreakHitResult _outhit))
      (:Is%20Valid
        (Development|SetHiddeninGame (.HitComponent (Collision|BreakHitResult _outhit)) false false))
      (:Is%20Not%20Valid
        _))
    (bind _hit_component (Variables|Default|GetHit%20Component)
      (:then
        (Development|SetHiddeninGame _hit_component true false))
      (:else
        _))
    (Variables|Default|SetHit%20Component (.HitComponent (Collision|BreakHitResult _outhit)))))

(event Custom|RaiseArm
  (Utilities|FlowControl|Sequence
    (:then_0
      (bind _alpha (Timeline|Raise PlayFromStart)
        (:Update
          (Transformation|SetRelativeLocationAndRotation (Variables|Default|GetLiftingArm) (Math|Vector|Lerp(Vector) "0.300000,13.000000,-27.000000" "27.000000,14.000000,-13.000000" _alpha) (Math|Rotator|Lerp(Rotator) "0.700000,-99.000000,-19.000000" "13.500000,-105.000000,-18.000000" _alpha true) false false))))
    (:then_1
      (Utilities|FlowControl|Delay 1.25)
      (Variables|Default|SetbRaiseArm true))))

(event Custom|Parting
  (bind _titlecard (Variables|Default|GetTitleCard))
  (Variables|Default|SetbIsBook true)
  (CameraFades|StartCameraFade (Game|GetPlayerCameraManager 0) 0.0 1.0 5.0 "(R=0.000000,G=0.000000,B=0.000000,A=1.000000)" true true)
  (Utilities|FlowControl|Delay 5.0)
  (CallFunction|NextCard "\"Yet I just can't get the right ticket\" 
")
  (Utilities|FlowControl|Delay 0.1)
  (UserInterface|Viewport|AddtoViewport _titlecard 0)
  (Utilities|FlowControl|Delay 4.0)
  (CallFunction|NextCard "“Farewell” 
I guess she would say")
  (Utilities|FlowControl|Delay 4.0)
  (CallFunction|NextCard "\"Farewell\"")
  (Utilities|FlowControl|Delay 4.0)
  (Widget|RemovefromParent _titlecard)
  (Audio|Components|Audio|Stop (Variables|Default|GetCardSfx))
  (Utilities|FlowControl|Delay 1.0)
  (bind _returnvalue (UserInterface|CreateWidget "/Game/5_Scene_Last/WB_EndSplash.WB_EndSplash_C"))
  (UserInterface|Viewport|AddtoViewport _returnvalue 0)
  (Utilities|FlowControl|Delay 4.0)
  (Widget|SetVisibility (Variables|/Game/5_Scene_Last/WB_EndSplash.WB_EndSplash_C|GetImage_28 _returnvalue) "Collapsed")
  (Utilities|FlowControl|Delay 1.0)
  (Widget|SetVisibility (Variables|/Game/5_Scene_Last/WB_EndSplash.WB_EndSplash_C|GetImage _returnvalue) "Visible")
  (Utilities|FlowControl|Delay 4.0)
  (Development|ExecuteConsoleCommand "exit" 0))

(event Custom|NextCard
  (params (InText :type Text))
  (bind _returnvalue (Audio|CreateSound2D "/Game/Sfx/Card.Card" 1.0 1.0 0.0 0))
  (bind _output_get (Variables|Default|SetCardSfx _returnvalue))
  (Audio|Components|Audio|Play _output_get 0.0)
  (Utilities|FlowControl|Delay 0.05)
  (Rendering|Components|TextRender|SetText (Variables|/Game/1_TrainStation/WB_TitleCard.WB_TitleCard_C|GetText (Variables|Default|GetTitleCard)) InText))

(event Input|EnhancedActionEvents|EnhancedInputActionIA_Space
  (params (ActionValue :type Boolean) (ElapsedSeconds :type Float%20%28double-precision%29) (TriggeredSeconds :type Float%20%28double-precision%29) (InputAction :type Input%20Action%20Object%20Reference :default "/Game/GameMode/Input/IA_Space.IA_Space"))
  (bind _returnvalue (Transformation|GetActorLocation))
  (bind _bisbook (Variables|Default|GetbIsBook))
  (:Triggered
    (if (not _bisbook)
      (Pawn|Input|AddMovementInput (Spline|FindDirectionClosesttoWorldLocation (Variables|Default|GetSpline) _returnvalue "World") 3.0 false)
      (if (< (Class|KismetMathLibrary|VectorDistanceSquared (Variables|Default|GetDestination) _returnvalue) (Variables|Default|GetThreshold))
        (CallFunction|Parting)
        (Audio|PlaySound2D "/Game/Sfx/5_TrainDeparting.5_TrainDeparting" 2.0 1.0 0.0 0 0))))
  (:Started
    (if (not _bisbook)
      (bind _returnvalue_2 (Audio|CreateSound2D "/Game/Sfx/15_PlatformWalking.15_PlatformWalking" 1.25 1.0 0.0 0))
      (bind _output_get (Variables|Default|SetWalking _returnvalue_2))
      (Audio|Components|Audio|Play _output_get (.OutItem (Utilities|Array|Random (Variables|Default|GetWalkTimes))))))
  (:Canceled
    (bind _walking (Variables|Default|GetWalking :!label _label)
      (:then
        (Audio|Components|Audio|Stop _walking))
      (:else)))
  (:Completed
    (goto _label)))

(event Input|EnhancedActionEvents|EnhancedInputActionIA_LeftClick
  (params (ActionValue :type Boolean) (ElapsedSeconds :type Float%20%28double-precision%29) (TriggeredSeconds :type Float%20%28double-precision%29) (InputAction :type Input%20Action%20Object%20Reference :default "/Game/GameMode/Input/IA_LeftClick.IA_LeftClick")))

(event Input|EnhancedActionEvents|EnhancedInputActionIA_Look
  (params (ActionValue :type Vector%202D%20Structure) (ElapsedSeconds :type Float%20%28double-precision%29) (TriggeredSeconds :type Float%20%28double-precision%29) (InputAction :type Input%20Action%20Object%20Reference :default "/Game/GameMode/Input/IA_Look.IA_Look"))
  (bind _returnvalue (Math|Float|MakeLiteralFloat 2.0))
  (bind _returnvalue_2 (* _returnvalue -1.0))
  (:Triggered
    (bind _output_get (Variables|Default|SetSmoothedVector (Math|Vector2D|MakeVector2D (Math|Float|Clamp(Float) (.x (Class|KismetMathLibrary|Vector2DInterpto (Variables|Default|GetSmoothedVector) (Math|Vector2D|MakeVector2D (.x ActionValue) (.y ActionValue)) (Utilities|Time|GetWorldDeltaSeconds) (Variables|Default|GetLookSmoothSpeed))) _returnvalue_2 _returnvalue) (Math|Float|Clamp(Float) (.y (Class|KismetMathLibrary|Vector2DInterpto (Variables|Default|GetSmoothedVector) (Math|Vector2D|MakeVector2D (.x ActionValue) (.y ActionValue)) (Utilities|Time|GetWorldDeltaSeconds) (Variables|Default|GetLookSmoothSpeed))) _returnvalue_2 _returnvalue))))
    (Pawn|Input|AddControllerYawInput (.x _output_get))
    (Pawn|Input|AddControllerPitchInput (.y _output_get)))
  (:Started
    (Variables|Default|SetbNotLooking false))
  (:Canceled
    (Variables|Default|SetbNotLooking true :!label _label))
  (:Completed
    (goto _label)))

(event EventBeginPlay
  (Utilities|FlowControl|Sequence
    (:then_0
      (bind _returnvalue (Actor|GetActorOfClass "/Game/2_Scene1/BP_Spline.BP_Spline_C"))
      (bind _output_get (Variables|Default|SetSpline (Variables|/Game/2_Scene1/BP_Spline.BP_Spline_C|GetSpline _returnvalue)))
      (Transformation|SetActorLocation (Math|Vector|MakeVector (.x (Spline|GetLocationatSplinePoint _output_get 0 "World")) (.y (Spline|GetLocationatSplinePoint _output_get 0 "World")) (.Z (Math|Vector|BreakVector (Transformation|GetActorLocation)))) false false)
      (Utilities|FlowControl|Delay 2.0)
      (CallFunction|NextCard "And I speak to myself:")
      (Utilities|FlowControl|Delay 0.1)
      (UserInterface|Viewport|AddtoViewport (Variables|Default|GetTitleCard) 0)
      (Utilities|FlowControl|Delay 4.0)
      (CallFunction|NextCard "\"See, it's time to go\"")
      (Utilities|FlowControl|Delay 4.0)
      (Audio|Components|Audio|Stop (Variables|Default|GetCardSfx))
      (Widget|RemovefromParent (Variables|Default|GetTitleCard)))
    (:then_1
      (bind _returnvalue_2 (UserInterface|CreateWidget "/Game/1_TrainStation/WB_TitleCard.WB_TitleCard_C"))
      (Variables|Default|SetTitleCard _returnvalue_2))
    (:then_2
      (bind _asbp_parting_game_instance (Utilities|Casting|CastToBP_PartingGameInstance (Game|GetGameInstance)))
      (bind _output_get_2 (Variables|Default|SetGameInstance _asbp_parting_game_instance))
      (bind _returnvalue_3 (Default|CreateSound _output_get_2 "/Game/Music/1_TrainStation_Original.1_TrainStation_Original" 2.5))
      (bind _output_get_3 (Variables|Default|SetMusic _returnvalue_3))
      (Audio|Components|Audio|FadeIn _output_get_3 5.0 1.0 1.0 "Linear" :!class /Script/Engine.AudioComponent)
      (Utilities|FlowControl|Delay 3.0)
      (bind _returnvalue_4 (Default|CreateSound _output_get_2 "/Game/Sfx/1_TrainStationAmbience.1_TrainStationAmbience" 1.0))
      (bind _output_get_4 (Variables|Default|SetAmbience _returnvalue_4))
      (Audio|Components|Audio|FadeIn _output_get_4 6.0 1.0 0.0 "Linear" :!class /Script/Engine.AudioComponent)
      (Utilities|FlowControl|Delay 3.0)
      (Audio|PlaySound2D "/Game/Sfx/15_TrainWhistle.15_TrainWhistle" 1.0 1.0 0.0 0 0))
    (:then_3
      (Components|Animation|PlayAnimation (Variables|Default|GetLiftingArm) "/Game/1_TrainStation/Arm_Idle.Arm_Idle" true)
      (bind _alpha (Timeline|Timeline Reverse)
        (:Update
          (Transformation|SetRelativeLocationAndRotation (Variables|Default|GetLiftingArm) (Math|Vector|Lerp(Vector) "0.300000,13.000000,-27.000000" "27.000000,14.000000,-13.000000" _alpha) (Math|Rotator|Lerp(Rotator) "0.700000,-99.000000,-19.000000" "13.500000,-105.000000,-18.000000" _alpha true) false false))))))

(event EventTick
  (params (DeltaSeconds :type Float%20%28single-precision%29))
  (if (Variables|Default|GetbNotLooking)
    (bind _output_get (Variables|Default|SetSmoothedVector (Math|Vector2D|MakeVector2D (.x (Class|KismetMathLibrary|Vector2DInterpto (Variables|Default|GetSmoothedVector) (Math|Vector2D|MakeVector2D 0.0 0.0) (Utilities|Time|GetWorldDeltaSeconds) (Variables|Default|GetLookSmoothSpeed))) (.y (Class|KismetMathLibrary|Vector2DInterpto (Variables|Default|GetSmoothedVector) (Math|Vector2D|MakeVector2D 0.0 0.0) (Utilities|Time|GetWorldDeltaSeconds) (Variables|Default|GetLookSmoothSpeed))))))
    (Pawn|Input|AddControllerYawInput (.x _output_get))
    (Pawn|Input|AddControllerPitchInput (.y _output_get))))

(fn ConstructionScript)

(fn HasTag
  (params (Component :type Actor%20Component%20Object%20Reference) (Tag :type Name))
  (for _array_element (Variables|/Script/Engine.ActorComponent|GetComponentTags Component)
    (if (== _array_element Tag)
      (return true)))
  (return false))