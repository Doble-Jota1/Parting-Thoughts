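; Player pawn for Scene 1 that keeps movement and view aligned to the level's BP_Spline paths, with look and move input disabled while IsBook is set.
; Each tick it finds the nearest spline, clamps camera yaw around that spline's direction, and pushes the player back when squared distance exceeds a threshold.
; When the nearest spline changes, the Transit timeline blends the yaw limits from the old direction to the new.
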(event Custom|TransitionSplines
  (params (Old :type Spline%20Component%20Object%20Reference) (New :type Spline%20Component%20Object%20Reference))
  (bind _returnvalue (Game|GetPlayerCameraManager 0))
  (bind _returnvalue_2 (Transformation|GetActorLocation))
  (bind _constrait (Variables|Default|GetConstrait))
  (bind _output_get (Variables|Default|SetOld (.yaw (Math|Rotator|MakeRotfromX (Spline|FindDirectionClosesttoWorldLocation Old _returnvalue_2 "World")))))
  (bind _output_get_2 (Variables|Default|SetNew (.yaw (Math|Rotator|MakeRotfromX (Spline|FindDirectionClosesttoWorldLocation New _returnvalue_2 "World")))))
  (bind _alpha (Timeline|Transit PlayFromStart)
    (:Update
      (Variables|/Script/Engine.PlayerCameraManager|SetViewYawMax _returnvalue (+ (Math|Float|Lerp _output_get _output_get_2 _alpha) _constrait))
      (Variables|/Script/Engine.PlayerCameraManager|SetViewYawMin _returnvalue (- (Math|Float|Lerp _output_get _output_get_2 _alpha) _constrait))
      (Development|PrintString "Transitioning"))
    (:Finished
      (Variables|Default|SetbInTransition false))))

(event Input|EnhancedActionEvents|EnhancedInputActionIA_Look
  (params (ActionValue :type Vector%202D%20Structure) (ElapsedSeconds :type Float%20%28double-precision%29) (TriggeredSeconds :type Float%20%28double-precision%29) (InputAction :type Input%20Action%20Object%20Reference :default "/Game/Blueprints/Input/IA_Look.IA_Look"))
  (if (not (Variables|Default|GetbIsBook))
    (Pawn|Input|AddControllerYawInput (.x ActionValue))
    (Pawn|Input|AddControllerPitchInput (.y ActionValue))))

(event Input|EnhancedActionEvents|EnhancedInputActionIA_Move
  (params (ActionValue :type Vector%202D%20Structure) (ElapsedSeconds :type Float%20%28double-precision%29) (TriggeredSeconds :type Float%20%28double-precision%29) (InputAction :type Input%20Action%20Object%20Reference :default "/Game/Blueprints/Input/IA_Move.IA_Move"))
  (if (not (Variables|Default|GetbIsBook))
    (Pawn|Input|AddMovementInput (Transformation|GetActorRightVector) (.x ActionValue) false)
    (Pawn|Input|AddMovementInput (Transformation|GetActorForwardVector) (.y ActionValue) false)))

(event EventBeginPlay
  (Utilities|FlowControl|Sequence
    (:then_0
      (bind _outactors (Actor|GetAllActorsOfClass "/Game/Scene1/BP_Spline.BP_Spline_C"))
      (Variables|Default|SetSplines _outactors)
      (bind _closest (CallFunction|GetClosestSpline))
      (Variables|Default|SetActiveSpline _closest)
      (Actor|Tick|SetActorTickEnabled true))))

(event EventTick
  (params (DeltaSeconds :type Float%20%28single-precision%29))
  (bind _returnvalue (Game|GetPlayerCameraManager 0))
  (bind _returnvalue_2 (Transformation|GetActorLocation))
  (bind _constrait (Variables|Default|GetConstrait))
  (Utilities|FlowControl|Sequence
    (:then_0
      (bind (_closest _distance) (CallFunction|GetClosestSpline))
      (Utilities|FlowControl|Sequence
        (:then_0
          (if (== _closest (Variables|Default|GetActiveSpline))
            (if (not (stale _output_get))
              (Variables|/Script/Engine.PlayerCameraManager|SetViewYawMax _returnvalue (+ (.yaw (Math|Rotator|MakeRotfromX (Spline|FindDirectionClosesttoWorldLocation (Variables|Default|GetActiveSpline) (Transformation|GetActorLocation) "World"))) _constrait))
              (Variables|/Script/Engine.PlayerCameraManager|SetViewYawMin _returnvalue (- (.yaw (Math|Rotator|MakeRotfromX (Spline|FindDirectionClosesttoWorldLocation (Variables|Default|GetActiveSpline) (Transformation|GetActorLocation) "World"))) _constrait)))
            (else
              (bind _output_get (Variables|Default|SetbInTransition true))
              (CallFunction|TransitionSplines (Variables|Default|GetActiveSpline) _closest)
              (Variables|Default|SetActiveSpline _closest))))
        (:then_1
          (if (> _distance (Variables|Default|GetDistance))
            (Pawn|Input|AddMovementInput (Math|Vector|Normalize (- _returnvalue_2 (Spline|FindLocationClosesttoWorldLocation (Variables|Default|GetActiveSpline) _returnvalue_2 "World"))) -2.0 false)))))))

(fn ConstructionScript)

(fn HasTag
  (params (Component :type Actor%20Component%20Object%20Reference) (Tag :type Name))
  (for _array_element (Variables|/Script/Engine.ActorComponent|GetComponentTags Component)
    (if (== _array_element Tag)
      (return true)))
  (return false))

(fn GetClosestSpline
  (bind _returnvalue (Transformation|GetActorLocation))
  (bind _splines (Variables|Default|GetSplines))
  (LocalVariables|SetSpline (Variables|/Game/Scene1/BP_Spline.BP_Spline_C|GetSpline (Utilities|Array|Get(acopy) _splines)))
  (for _array_element _splines
    (if (< (Class|KismetMathLibrary|VectorDistanceSquared (Spline|FindLocationClosesttoWorldLocation (Variables|/Game/Scene1/BP_Spline.BP_Spline_C|GetSpline _array_element) _returnvalue "World") _returnvalue) (LocalVariables|GetMin))
      (LocalVariables|SetMin (Class|KismetMathLibrary|VectorDistanceSquared (Spline|FindLocationClosesttoWorldLocation (Variables|/Game/Scene1/BP_Spline.BP_Spline_C|GetSpline _array_element) _returnvalue "World") _returnvalue))
      (LocalVariables|SetSpline (Variables|/Game/Scene1/BP_Spline.BP_Spline_C|GetSpline _array_element))))
  (return (LocalVariables|GetSpline) (LocalVariables|GetMin)))