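; Player for a walking scene with narrative title cards, moved along a tagged spline with Space and free to look around outside cards.
; BeginPlay snaps to the spline, shows an opening card and starts ambience.
; The Cards event plays dialogue cards, locks look input and pans the camera through chained timelines.
; Tick then moves the Figure along its own spline while player and Figure speed up, before TrainStation_LastScene loads on a delay.
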(event Custom|Cards
  (bind _returnvalue (Game|GetPlayerController 0))
  (bind _figurespline (Variables|Default|GetFigureSpline))
  (bind _titlecard (Variables|Default|GetTitleCard))
  (bind _returnvalue_2 (Spline|GetLocationatSplinePoint _figurespline 0 "World"))
  (bind _returnvalue_3 (Pawn|GetControlRotation _returnvalue :!class /Script/Engine.Controller))
  (Variables|Default|SetbIsBook true)
  (Audio|Components|Audio|Stop (Variables|Default|GetTypewriter))
  (CallFunction|NextCard "\"Thanks for walking me back\"")
  (Utilities|FlowControl|Delay 0.1)
  (UserInterface|Viewport|AddtoViewport _titlecard 0)
  (Utilities|FlowControl|Delay 4.0)
  (CallFunction|NextCard "“I guess I’ll see you later” 
She says")
  (Utilities|FlowControl|Delay 4.0)
  (CallFunction|NextCard "I wish I could follow 
But the body won’t turn")
  (Utilities|FlowControl|Delay 4.0)
  (Widget|RemovefromParent _titlecard)
  (Audio|Components|Audio|Stop (Variables|Default|GetCardSfx))
  (Variables|Default|SetbIsBook false)
  (Utilities|FlowControl|Sequence
    (:then_0
      (Transformation|SetActorLocation (Variables|Default|GetFigure) (Math|Vector|MakeVector (.x _returnvalue_2) (.y _returnvalue_2) 1476.65554) false false)
      (Actor|Tick|SetActorTickEnabled true)
      (Utilities|FlowControl|Sequence
        (:then_0
          (Utilities|FlowControl|Delay 2.0)
          (Utilities|FlowControl|Gate true) ; enters at Open
        )
        (:then_1
          (Utilities|FlowControl|Delay 3e+01)
          (bind _asbp_parting_game_instance (Utilities|Casting|CastToBP_PartingGameInstance (Game|GetGameInstance)))
          (Default|LoadLevel _asbp_parting_game_instance "/Game/Scene_Last/TrainStation_LastScene.TrainStation_LastScene"))))
    (:then_1
      (bind _alpha (Timeline|Orient PlayFromStart)
        (:Update
          (Pawn|SetControlRotation _returnvalue (Math|Rotator|MakeRotator (.roll _returnvalue_3) (Math|Float|Lerp 0.0 -8.0 _alpha) (Math|Float|Lerp 0.0 48.0 _alpha))))
        (:Finished
          (bind _output_get (Variables|Default|SetTemp (.yaw _returnvalue_3)))
          (bind _alpha_2 (Timeline|Slow PlayFromStart)
            (:Update
              (Pawn|SetControlRotation _returnvalue (Math|Rotator|MakeRotator (.roll _returnvalue_3) (.pitch _returnvalue_3) (Math|Float|Lerp _output_get 72.0 _alpha_2))))
            (:Finished
              (bind _output_get_2 (Variables|Default|SetTemp (.yaw _returnvalue_3)))
              (bind _output_get_3 (Variables|Default|SetTemp2 (.pitch _returnvalue_3)))
              (bind _alpha_3 (Timeline|Timeline PlayFromStart)
                (:Update
                  (Pawn|SetControlRotation (Game|GetPlayerController 0) (Math|Rotator|MakeRotator 0.0 (Math|Float|Lerp _output_get_3 2.0 _alpha_3) (Math|Float|Lerp _output_get_2 8e+01 _alpha_3))))))))))
    (:then_2
      (Utilities|FlowControl|Gate false) ; enters at Close
    )))

(event Custom|NextCard
  (params (InText :type Text))
  (bind _returnvalue (Audio|CreateSound2D "/Game/Sfx/Card.Card" 1.0 1.0 0.0 0))
  (bind _output_get (Variables|Default|SetCardSfx _returnvalue))
  (Audio|Components|Audio|Play _output_get 0.0)
  (Utilities|FlowControl|Delay 0.05)
  (Rendering|Components|TextRender|SetText (Variables|/Game/TrainStation/WB_TitleCard.WB_TitleCard_C|GetText (Variables|Default|GetTitleCard)) InText))

(event Input|EnhancedActionEvents|EnhancedInputActionIA_Space
  (params (ActionValue :type Boolean) (ElapsedSeconds :type Float%20%28double-precision%29) (TriggeredSeconds :type Float%20%28double-precision%29) (InputAction :type Input%20Action%20Object%20Reference :default "/Game/Blueprints/Input/IA_Space.IA_Space"))
  (if (not (Variables|Default|GetbIsBook))
    (Pawn|Input|AddMovementInput (Spline|FindDirectionClosesttoWorldLocation (Variables|Default|GetActiveSpline) (Transformation|GetActorLocation) "World") 5.0 false)))

(event Input|EnhancedActionEvents|EnhancedInputActionIA_Look
  (params (ActionValue :type Vector%202D%20Structure) (ElapsedSeconds :type Float%20%28double-precision%29) (TriggeredSeconds :type Float%20%28double-precision%29) (InputAction :type Input%20Action%20Object%20Reference :default "/Game/Blueprints/Input/IA_Look.IA_Look"))
  (if (not (Variables|Default|GetbIsBook))
    (Utilities|FlowControl|Gate false
      (:Exit
        (Pawn|Input|AddControllerYawInput (.x ActionValue))
        (Pawn|Input|AddControllerPitchInput (.y ActionValue))))))

(event EventBeginPlay
  (bind _returnvalue (Transformation|GetActorLocation))
  (Utilities|FlowControl|Sequence
    (:then_0
      (bind _outactors (Actor|GetAllActorsOfClasswithTag "/Game/Scene1/BP_Spline.BP_Spline_C" "Player"))
      (bind _output_get (Variables|Default|SetActiveSpline (Variables|/Game/Scene1/BP_Spline.BP_Spline_C|GetSpline (Utilities|Array|Get(acopy) _outactors))))
      (bind _outactors_2 (Actor|GetAllActorsOfClasswithTag "/Game/Scene1/BP_Spline.BP_Spline_C" "Figure"))
      (Variables|Default|SetFigureSpline (Variables|/Game/Scene1/BP_Spline.BP_Spline_C|GetSpline (Utilities|Array|Get(acopy) _outactors_2)))
      (Transformation|SetActorLocation (Math|Vector|MakeVector (.x (Spline|FindLocationClosesttoWorldLocation _output_get _returnvalue "World")) (.y (Spline|FindLocationClosesttoWorldLocation _output_get _returnvalue "World")) (.Z (Math|Vector|BreakVector _returnvalue))) false false)
      (bind _outactors_3 (Actor|GetAllActorsOfClasswithTag "/Script/Engine.StaticMeshActor" "Figure"))
      (Variables|Default|SetFigure (Utilities|Array|Get(acopy) _outactors_3)))
    (:then_1
      (bind _returnvalue_2 (UserInterface|CreateWidget "/Game/TrainStation/WB_TitleCard.WB_TitleCard_C"))
      (bind _output_get_2 (Variables|Default|SetTitleCard _returnvalue_2))
      (Variables|Default|SetbIsBook true)
      (CallFunction|NextCard "“Let’s go back together” 
She says")
      (UserInterface|Viewport|AddtoViewport _output_get_2 0)
      (Utilities|FlowControl|Delay 4.0)
      (Widget|RemovefromParent _output_get_2)
      (Audio|Components|Audio|Stop (Variables|Default|GetCardSfx))
      (Variables|Default|SetbIsBook false)
      (bind _returnvalue_3 (Audio|CreateSound2D "/Game/Sfx/2_Typewriter.2_Typewriter" 1.0 1.0 0.0 0))
      (bind _output_get_3 (Variables|Default|SetTypewriter _returnvalue_3))
      (Audio|Components|Audio|Play _output_get_3 0.0)
      (Audio|PlaySound2D "/Game/Sfx/2_MaggieMoAmbience.2_MaggieMoAmbience" 4.0 1.0 0.0 0 0)
      (Audio|PlaySound2D "/Game/Music/2_MaggieMo.2_MaggieMo" 24.0 1.0 0.0 0 0))))

(event EventTick
  (params (DeltaSeconds :type Float%20%28single-precision%29))
  (bind _figure (Variables|Default|GetFigure))
  (bind _returnvalue (Transformation|GetActorLocation _figure))
  (Transformation|SetActorLocationAndRotation _figure (Math|Vector|MakeVector (.x (+ _returnvalue (* (Spline|FindDirectionClosesttoWorldLocation (Variables|Default|GetFigureSpline) _returnvalue "World") (Variables|Default|GetFigureSpeed)))) (.y (+ _returnvalue (* (Spline|FindDirectionClosesttoWorldLocation (Variables|Default|GetFigureSpline) _returnvalue "World") (Variables|Default|GetFigureSpeed)))) 1476.65554) (Math|Rotator|FindLookatRotation _returnvalue (* (Spline|FindDirectionClosesttoWorldLocation (Variables|Default|GetFigureSpline) _returnvalue "World") (Variables|Default|GetFigureSpeed))))
  (Utilities|FlowControl|Gate true
    (:Exit
      (Pawn|Input|AddMovementInput (Spline|FindDirectionClosesttoWorldLocation (Variables|Default|GetActiveSpline) (Transformation|GetActorLocation) "World") (Variables|Default|GetScale%20Value) false)
      (Variables|Default|SetScale%20Value (Math|Float|Clamp(Float) (+ (Variables|Default|GetScale%20Value) 0.001) 0.0 0.5))
      (Variables|Default|SetFigureSpeed (Math|Float|Clamp(Float) (+ (Variables|Default|GetFigureSpeed) 0.04) 0.0 3e+01)))))

(fn ConstructionScript)