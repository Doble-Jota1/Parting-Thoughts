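; BP_Forest procedurally scatters instanced trees within its Bounds component, with separate events to sample points, generate and delete.
; SamplePoints picks random points, rejecting those near BP_Spline actors or inside child mesh exclusion boxes, and logs failures.
; GenerateTrees builds each stored point into a randomly sized trunk with four thinner surrounding pieces, plus three tapering layers of randomly scattered leaves.
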(event Custom|SamplePoints
  (bind _bounds (Variables|Default|GetBounds))
  (bind _returnvalue (Transformation|GetWorldScale _bounds))
  (Rendering|Debug|FlushPersistentDebugLines)
  (Variables|Default|SetCounter 0)
  (Utilities|Array|Clear (Variables|Default|GetExclusions))
  (for _array_element (Components|GetChildrenComponents (Variables|Default|GetDefaultSceneRoot) false)
    (if (not (Math|Boolean|ORBoolean (== _array_element (Variables|Default|GetBounds)) (== _array_element (Variables|Default|GetTrees)) (== _array_element (Variables|Default|GetLeaves))))
      (bind _asstatic_mesh_component (Utilities|Casting|CastToStaticMeshComponent _array_element))
      (Utilities|Array|Add (Variables|Default|GetExclusions) _asstatic_mesh_component)))
  (bind _outactors (Actor|GetAllActorsOfClass "/Game/2_Scene1/BP_Spline.BP_Spline_C"))
  (bind _output_get (Variables|Default|SetSplines _outactors))
  (for _index (range 0 (Variables|Default|GetNumTrees))
    (bind _output_get_2 (Variables|Default|SetbSuccess false))
    (Utilities|FlowControl|ForLoopwithBreak 0 (Variables|Default|GetTries) :!label _label
      (:LoopBody
        (bind _output_get_3 (Variables|Default|SetPoint (+ (Math|Vector|MakeVector (Math|Random|RandomFloatinRange (* (.x _returnvalue) -5e+01) (* (.x _returnvalue) 5e+01)) (Math|Random|RandomFloatinRange (* (.y _returnvalue) -5e+01) (* (.y _returnvalue) 5e+01)) 0.0) (Transformation|GetWorldLocation (Variables|Default|GetBounds)))))
        (bind _output_get_4 (Variables|Default|SetbInner true))
        (bind _array_element_2 (Utilities|Array|ForEachLoopwithBreak _output_get :!label _label_2)
          (:LoopBody
            (if (not (> (Class|KismetMathLibrary|VectorDistanceSquared (Spline|FindLocationClosesttoWorldLocation (Variables|/Game/2_Scene1/BP_Spline.BP_Spline_C|GetSpline _array_element_2) _output_get_3 "World") _output_get_3) (Variables|Default|GetMargin)))
              (Variables|Default|SetbInner false)
              (goto _label_2 Break)))
          (:Completed
            (bind _array_element_3 (Utilities|Array|ForEachLoopwithBreak (Variables|Default|GetExclusions) :!label _label_3)
              (:LoopBody
                (if (Math|Boolean|ANDBoolean (> (.x (- (Variables|Default|GetPoint) "")) (+ (* (.x (Transformation|GetWorldScale _array_element_3)) -5e+01) (.x (Math|Vector|NegateVector (Transformation|GetWorldLocation _array_element_3))))) (< (.x (- (Variables|Default|GetPoint) "")) (+ (* (.x (Transformation|GetWorldScale _array_element_3)) 5e+01) (.x (Math|Vector|NegateVector (Transformation|GetWorldLocation _array_element_3))))) (> (.y (- (Variables|Default|GetPoint) "")) (+ (* (.y (Transformation|GetWorldScale _array_element_3)) -5e+01) (.Y (Math|Vector|BreakVector (Transformation|GetWorldLocation _array_element_3))))) (< (.y (- (Variables|Default|GetPoint) "")) (+ (* (.y (Transformation|GetWorldScale _array_element_3)) 5e+01) (.Y (Math|Vector|BreakVector (Transformation|GetWorldLocation _array_element_3))))))
                  (Variables|Default|SetbInner false)
                  (goto _label_3 Break)))
              (:Completed
                (Variables|Default|SetbSuccess _output_get_4)
                (goto _label Break))))))
      (:Completed
        (if _output_get_2
          (Utilities|Array|Add (Variables|Default|GetPoints) _output_get_3)
          (else
            (Development|PrintString "FAILED" true true "(R=1.000000,G=0.000000,B=0.009138,A=1.000000)")
            (Math|Integer|IncrementInt (Variables|Default|GetCounter)))))))
  (Development|PrintText (Utilities|Text|FormatText "{num} failed" (Variables|Default|GetCounter))))

(event Custom|GenerateTrees
  (bind _returnvalue (Math|Random|RandomFloatinRange 0.0 3.6e+02))
  (bind _trees (Variables|Default|GetTrees))
  (Components|InstancedStaticMesh|ClearInstances (Variables|Default|GetTrees))
  (for _array_element (Variables|Default|GetPoints)
    (bind _output_get (Variables|Default|SetHeight (Math|Random|RandomFloatinRange 2.0 8.0)))
    (bind _output_get_2 (Variables|Default|SetWidth (Math|Random|RandomFloatinRange 0.05 0.3)))
    (Components|InstancedStaticMesh|AddInstance (Variables|Default|GetTrees) (Math|Transform|MakeTransform _array_element "0, 0, 0" (Math|Vector|MakeVector _output_get_2 _output_get_2 _output_get)) true)
    (Components|InstancedStaticMesh|AddInstance _trees (Math|Transform|MakeTransform (+ _array_element (Math|Vector|MakeVector (+ (/ (Variables|Default|GetWidth) 0.01) (/ (/ (Variables|Default|GetWidth) 0.01) 2.0)) (/ (/ (Variables|Default|GetWidth) 0.01) 2.0) 0.0)) "0, 0, 0" (Math|Vector|MakeVector (/ (Variables|Default|GetWidth) 2.0) (/ (Variables|Default|GetWidth) 2.0) (* (Variables|Default|GetHeight) (Math|Random|RandomFloatinRange 0.2 4.0)))) true)
    (Components|InstancedStaticMesh|AddInstance _trees (Math|Transform|MakeTransform (+ _array_element (Math|Vector|MakeVector (* (/ (/ (Variables|Default|GetWidth) 0.01) 2.0) -1.0) (+ (/ (Variables|Default|GetWidth) 0.01) (/ (/ (Variables|Default|GetWidth) 0.01) 2.0)) 0.0)) "0, 0, 0" (Math|Vector|MakeVector (/ (Variables|Default|GetWidth) 2.0) (/ (Variables|Default|GetWidth) 2.0) (* (Variables|Default|GetHeight) (Math|Random|RandomFloatinRange 0.2 4.0)))) true)
    (Components|InstancedStaticMesh|AddInstance _trees (Math|Transform|MakeTransform (+ _array_element (Math|Vector|MakeVector (* (+ (/ (Variables|Default|GetWidth) 0.01) (/ (/ (Variables|Default|GetWidth) 0.01) 2.0)) -1.0) (* (/ (/ (Variables|Default|GetWidth) 0.01) 2.0) -1.0) 0.0)) "0, 0, 0" (Math|Vector|MakeVector (/ (Variables|Default|GetWidth) 2.0) (/ (Variables|Default|GetWidth) 2.0) (* (Variables|Default|GetHeight) (Math|Random|RandomFloatinRange 0.2 4.0)))) true)
    (Components|InstancedStaticMesh|AddInstance _trees (Math|Transform|MakeTransform (+ _array_element (Math|Vector|MakeVector (/ (/ (Variables|Default|GetWidth) 0.01) 2.0) (* (+ (/ (Variables|Default|GetWidth) 0.01) (/ (/ (Variables|Default|GetWidth) 0.01) 2.0)) -1.0) 0.0)) "0, 0, 0" (Math|Vector|MakeVector (/ (Variables|Default|GetWidth) 2.0) (/ (Variables|Default|GetWidth) 2.0) (* (Variables|Default|GetHeight) (Math|Random|RandomFloatinRange 0.2 4.0)))) true)
    (bind _output_get_3 (Variables|Default|SetTempStep (* (Utilities|Operators|Divide (Variables|Default|GetHeight) 4.0 0.005) 4.0)))
    (for _index (range 1 3)
      (for _index_2 (range 0 (* (- 4 _index) (Variables|Default|GetLeavesPerLayer)))
        (bind _output_get_4 (Variables|Default|SetTemp (* (Math|Random|RandomFloatinRange 0.5 0.9) (- 1.0 (* _index 0.2)))))
        (Components|InstancedStaticMesh|AddInstance (Variables|Default|GetLeaves) (Math|Transform|MakeTransform (+ (Math|Vector|MakeVector (* (* (Math|Float|Lerp (* (- 1.0 (* _index 0.3)) (Variables|Default|GetRTop)) (* (- 1.0 (* _index 0.3)) (Variables|Default|GetRBottom)) (Math|Random|RandomFloatinRange 0.0 0.8)) (Math|Float|Sqrt (Math|Random|RandomFloat))) (Math|Trig|Cos(Degrees) _returnvalue)) (* (* (Math|Float|Lerp (* (- 1.0 (* _index 0.3)) (Variables|Default|GetRTop)) (* (- 1.0 (* _index 0.3)) (Variables|Default|GetRBottom)) (Math|Random|RandomFloatinRange 0.0 0.8)) (Math|Float|Sqrt (Math|Random|RandomFloat))) (Math|Trig|Sin(Degrees) _returnvalue)) (+ (* _index _output_get_3 (Math|Random|RandomFloatinRange 0.9 1.1)) (Math|Random|RandomFloatinRange 0.0 _output_get_3))) _array_element) "0, 0, 0" (Math|Vector|MakeVector _output_get_4 _output_get_4 (* (Math|Random|RandomFloatinRange 1.0 3.0) (- 1.0 (* _index 0.2))))) true)))))

(event Custom|DeleteTrees
  (Components|InstancedStaticMesh|ClearInstances (Variables|Default|GetTrees)))

(fn ConstructionScript)