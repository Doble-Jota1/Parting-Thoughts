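; BP_Rocks procedurally scatters rock instances along every BP_Spline actor in the level.
; Its construction script samples each spline at SampleInterval steps, spawning a random number of instances across three instanced static mesh components.
; Instances get random distance jitter, height, sideways offset from the spline direction crossed with up, and per-axis scale, but no random rotation.
; The event graph is empty.
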(event EventBeginPlay)

(event Collision|EventActorBeginOverlap
  (params (OtherActor :type Actor%20Object%20Reference)))

(event EventTick
  (params (DeltaSeconds :type Float%20%28single-precision%29)))

(fn ConstructionScript
  (bind _offsetvertical (Variables|Default|GetOffsetVertical))
  (bind _sampleinterval (Variables|Default|GetSampleInterval))
  (bind _sizemin (Variables|Default|GetSizeMin))
  (bind _sizemax (Variables|Default|GetSizeMax))
  (bind _offsethorizontal (Variables|Default|GetOffsetHorizontal))
  (bind _returnvalue (/ _sampleinterval 2))
  (bind _outactors (Actor|GetAllActorsOfClass "/Game/2_Scene1/BP_Spline.BP_Spline_C"))
  (bind _output_get (LocalVariables|SetSplines _outactors))
  (for _array_element _output_get
    (for _index (range 0 (/ (Spline|GetSplineLength (Variables|/Game/2_Scene1/BP_Spline.BP_Spline_C|GetSpline _array_element)) _sampleinterval))
      (bind _output_get_2 (LocalVariables|SetTemp (Math|Random|RandomIntegerinRange 0 (Variables|Default|GetRocksPerSample))))
      (for _index_2 (range 0 _output_get_2)
        (Components|InstancedStaticMesh|AddInstance (Utilities|Select :Index (Math|Random|RandomIntegerinRange 0 2) :Option%200 (Variables|Default|GetInstancedStaticMesh) :Option%201 (Variables|Default|GetInstancedStaticMesh1) :Option%202 (Variables|Default|GetInstancedStaticMesh2)) (Math|Transform|MakeTransform (+ (.location (Spline|GetTransformatDistanceAlongSpline (Variables|/Game/2_Scene1/BP_Spline.BP_Spline_C|GetSpline _array_element) (+ (Math|Conversions|ToFloat(Integer) (* _index _sampleinterval)) (Math|Random|RandomFloatinRange (* _returnvalue -1.0) _returnvalue)) "World" false)) (Math|Vector|MakeVector 0.0 0.0 (+ (Math|Random|RandomFloatinRange _offsetvertical (* _offsetvertical -1.0)) (Variables|Default|GetHeight))) (* (Math|Vector|CrossProduct (Spline|GetDirectionatDistanceAlongSpline (Variables|/Game/2_Scene1/BP_Spline.BP_Spline_C|GetSpline _array_element) (+ (Math|Conversions|ToFloat(Integer) (* _index _sampleinterval)) (Math|Random|RandomFloatinRange (* _returnvalue -1.0) _returnvalue)) "World") "0.000000,0.000000,1.000000") (Math|Random|RandomFloatinRange _offsethorizontal (* _offsethorizontal -1.0)))) "0, 0, 0" (Math|Vector|MakeVector (Math|Random|RandomFloatinRange _sizemin _sizemax) (Math|Random|RandomFloatinRange _sizemin _sizemax) (Math|Random|RandomFloatinRange _sizemin _sizemax))) true)))))