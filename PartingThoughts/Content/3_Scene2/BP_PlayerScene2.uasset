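; First-person player for Scene 2 that walks a looping path and can click a BP_Munin to start a scripted sitting sequence.
; Holding Space moves along BP_Spline, easing speed down before bends via a look-ahead direction dot product and wrapping at the end.
; A per-tick camera trace drives Munin highlighting.
; Clicking locks input, then chained timelines move the view into the seat, zoom out to Munin's camera, animate its hair and spawn BP_Jerry.
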(event Custom|Highlight
  (params (Comp :type Primitive%20Component%20Object%20Reference) (bHighlight :type Boolean))
  (bind _asbp_munin (Utilities|Casting|CastToBP_Munin (Components|GetOwner Comp)))
  (Default|Highlight _asbp_munin bHighlight))

(event Input|EnhancedActionEvents|EnhancedInputActionIA_Look
  (params (ActionValue :type Vector%202D%20Structure) (ElapsedSeconds :type Float%20%28double-precision%29) (TriggeredSeconds :type Float%20%28double-precision%29) (InputAction :type Input%20Action%20Object%20Reference :default "/Game/GameMode/Input/IA_Look.IA_Look"))
  (if (not (Variables|Default|GetbIsBook))
    (Pawn|Input|AddControllerYawInput (.x ActionValue))
    (Pawn|Input|AddControllerPitchInput (.y ActionValue))))

(event Input|EnhancedActionEvents|EnhancedInputActionIA_LeftClick
  (params (ActionValue :type Boolean) (ElapsedSeconds :type Float%20%28double-precision%29) (TriggeredSeconds :type Float%20%28double-precision%29) (InputAction :type Input%20Action%20Object%20Reference :default "/Game/GameMode/Input/IA_LeftClick.IA_LeftClick"))
  (bind _returnvalue (Game|GetPlayerController 0))
  (bind _returnvalue_2 (Game|GetPlayerController 0))
  (bind _firstpersoncamera (Variables|Default|GetFirstPersonCamera))
  (:Completed
    (if (not (Variables|Default|GetbIsBook))
      (bind _hit_component (Variables|Default|GetHit%20Component)
        (:then
          (Variables|Default|SetbIsBook true)
          (Actor|Tick|SetActorTickEnabled false)
          (Utilities|FlowControl|Sequence
            (:then_0
              (bind _asbp_munin (Utilities|Casting|CastToBP_Munin (Components|GetOwner _hit_component)))
              (Components|Timeline|SetPlayRate (Variables|Default|GetPreSit) 0.5)
              (bind _output_get (Variables|Default|SetStartRot (Pawn|GetControlRotation _returnvalue_2 :!class /Script/Engine.Controller)))
              (bind _output_get_2 (Variables|Default|SetStartLoc (Transformation|GetActorLocation)))
              (bind _alpha (Timeline|PreSit PlayFromStart)
                (:Update
                  (Pawn|SetControlRotation _returnvalue_2 (Math|Rotator|Lerp(Rotator) _output_get (Transformation|GetWorldRotation (Variables|/Game/3_Scene2/BP_Munin.BP_Munin_C|GetHeadRef _asbp_munin)) _alpha true))
                  (Transformation|SetActorLocation (Math|Vector|Lerp(Vector) _output_get_2 (Transformation|GetWorldLocation (Variables|/Game/3_Scene2/BP_Munin.BP_Munin_C|GetBodyRef _asbp_munin)) _alpha) false false))
                (:Finished
                  (Components|Timeline|SetPlayRate (Variables|Default|GetSit2) 0.75)
                  (bind _output_get_3 (Variables|Default|SetStartRot (Transformation|GetWorldRotation (Variables|/Game/3_Scene2/BP_Munin.BP_Munin_C|GetHeadRef _asbp_munin))))
                  (bind _output_get_4 (Variables|Default|SetStartLoc (Transformation|GetWorldLocation (Variables|/Game/3_Scene2/BP_Munin.BP_Munin_C|GetBodyRef _asbp_munin))))
                  (bind _alpha_2 (Timeline|Sit2 PlayFromStart)
                    (:Update
                      (Pawn|SetControlRotation (Game|GetPlayerController 0) (Math|Rotator|Lerp(Rotator) _output_get_3 "2.000000,82.000000,-2.000000" _alpha_2 true))
                      (Transformation|SetActorLocation (Math|Vector|Lerp(Vector) _output_get_4 (- _output_get_4 "4.000000,20.000000,15.000000") _alpha_2) false false))
                    (:Finished
                      (Components|Timeline|SetPlayRate (Variables|Default|GetSit3) 0.9)
                      (bind _output_get_5 (Variables|Default|SetStartRot "2.000000,82.000000,-2.000000"))
                      (bind _output_get_6 (Variables|Default|SetStartLoc (Transformation|GetActorLocation)))
                      (bind _alpha_3 (Timeline|Sit3 PlayFromStart)
                        (:Update
                          (Pawn|SetControlRotation (Game|GetPlayerController 0) (Math|Rotator|Lerp(Rotator) _output_get_5 (Transformation|GetWorldRotation (Variables|/Game/3_Scene2/BP_Munin.BP_Munin_C|GetHeadRef1 _asbp_munin)) _alpha_3 true))
                          (Transformation|SetActorLocation (Math|Vector|Lerp(Vector) _output_get_6 (- _output_get_6 "0.000000,-2.000000,0.000000") _alpha_3) false false))
                        (:Finished
                          (Components|Timeline|SetPlayRate (Variables|Default|GetSit4) 0.8)
                          (bind _output_get_7 (Variables|Default|SetStartRot (Transformation|GetWorldRotation (Variables|/Game/3_Scene2/BP_Munin.BP_Munin_C|GetHeadRef1 _asbp_munin))))
                          (bind _output_get_8 (Variables|Default|SetStartLoc (Transformation|GetActorLocation)))
                          (bind _alpha_4 (Timeline|Sit4 PlayFromStart)
                            (:Update
                              (Pawn|SetControlRotation (Game|GetPlayerController 0) (Math|Rotator|Lerp(Rotator) _output_get_7 "2.000000,94.000000,1.000000" _alpha_4 true))
                              (Transformation|SetActorLocation (Math|Vector|Lerp(Vector) _output_get_8 (- _output_get_8 "-5.000000,8.000000,3.000000") _alpha_4) false false))
                            (:Finished
                              (Utilities|FlowControl|Sequence
                                (:then_0
                                  (Components|Timeline|SetPlayRate (Variables|Default|GetZoomOut) 0.2)
                                  (bind _output_get_9 (Variables|Default|SetStartRot (Pawn|GetControlRotation _returnvalue :!class /Script/Engine.Controller)))
                                  (bind _output_get_10 (Variables|Default|SetStartLoc (Transformation|GetWorldLocation _firstpersoncamera)))
                                  (bind _alpha_5 (Timeline|ZoomOut PlayFromStart)
                                    (:Update
                                      (Transformation|SetWorldLocation _firstpersoncamera (Math|Vector|Lerp(Vector) _output_get_10 (.location (Transformation|GetWorldTransform (Variables|/Game/3_Scene2/BP_Munin.BP_Munin_C|GetCamera _asbp_munin))) _alpha_5) false false)
                                      (Pawn|SetControlRotation _returnvalue (Math|Rotator|Lerp(Rotator) _output_get_9 (.rotation (Transformation|GetWorldTransform (Variables|/Game/3_Scene2/BP_Munin.BP_Munin_C|GetCamera _asbp_munin))) _alpha_5 true)))))
                                (:then_1
                                  (Utilities|FlowControl|Delay 4.0)
                                  (Rendering|SetVisibility (Variables|/Game/3_Scene2/BP_Munin.BP_Munin_C|GetHead _asbp_munin) false false)
                                  (Components|Timeline|SetPlayRate (Variables|Default|GetHair) 0.5)
                                  (bind _alpha_6 (Timeline|Hair PlayFromStart)
                                    (:Update
                                      (Transformation|SetRelativeLocationAndRotation (Variables|/Game/3_Scene2/BP_Munin.BP_Munin_C|GetHair _asbp_munin) (Math|Vector|Lerp(Vector) "19.350000,-14.550000,96.000000" "15.780000,-14.550000,90.560000" _alpha_6) (Math|Rotator|Lerp(Rotator) "0, 0, 0" "47.300000,0.000000,0.000000" _alpha_6 true) false false)
                                      (Transformation|SetRelativeRotation (Variables|/Game/3_Scene2/BP_Munin.BP_Munin_C|GetBodyRef _asbp_munin) (Math|Rotator|Lerp(Rotator) "0, 0, 0" "2.000000,0.000000,0.000000" _alpha_6 true) false false))))
                                (:then_2
                                  (Game|SpawnActorfromClass "/Game/3_Scene2/BP_Jerry.BP_Jerry_C" (Math|Transform|MakeTransform (+ (Transformation|GetActorLocation _asbp_munin) "0.500000,0.000000,-3.000000") "0, 0, 0" "1.000000,1.000000,1.000000") "AlwaysSpawn" "MultiplyWithRoot" 0 0))))))))))))
            (:then_1
              (Collision|SetCollisionEnabled (Variables|Collision|GetCapsuleComponent) "NoCollision")
              (CallFunction|Highlight _hit_component false))))
        (:else)))))

(event Input|EnhancedActionEvents|EnhancedInputActionIA_Space
  (params (ActionValue :type Boolean) (ElapsedSeconds :type Float%20%28double-precision%29) (TriggeredSeconds :type Float%20%28double-precision%29) (InputAction :type Input%20Action%20Object%20Reference :default "/Game/GameMode/Input/IA_Space.IA_Space"))
  (bind _returnvalue (Transformation|GetActorLocation))
  (bind _returnvalue_2 (Transformation|GetActorLocation))
  (bind _bisbook (Variables|Default|GetbIsBook))
  (bind _activespline (Variables|Default|GetActiveSpline))
  (bind _returnvalue_3 (Spline|FindDirectionClosesttoWorldLocation _activespline _returnvalue "World"))
  (bind _returnvalue_4 (Spline|GetLocationatSplinePoint _activespline 0 "World"))
  (bind _z (Math|Vector|BreakVector _returnvalue_2))
  (bind _returnvalue_5 (Spline|FindLocationClosesttoWorldLocation _activespline _returnvalue "World"))
  (:Triggered
    (if (not _bisbook)
      (Transformation|SetActorLocation (Math|Vector|MakeVector (.x _returnvalue_5) (.y _returnvalue_5) _z) false false)
      (bind _output_get (Variables|Default|SetCurrentSpeed (Math|Interpolation|FInterpTo (stale _output_get) (Math|Float|SelectFloat 0.05 0.3 (< (/ (+ (Math|Vector|DotProduct _returnvalue_3 (Spline|GetDirectionatDistanceAlongSpline _activespline (+ (Class|SplineComponent|GetDistanceAlongSplineatLocation _activespline _returnvalue "World") (Variables|Default|GetLookahead)) "World")) 1.0) 2.0) 0.7)) (Utilities|Time|GetWorldDeltaSeconds) 4.0)))
      (Pawn|Input|AddMovementInput _returnvalue_3 _output_get false)
      (if (not (> (Class|KismetMathLibrary|VectorDistanceSquared (Spline|GetLocationatSplinePoint _activespline (Spline|GetNumberOfSplinePoints _activespline) "World") _returnvalue_2) 8e+03))
        (Transformation|SetActorLocation (Math|Vector|MakeVector (.x _returnvalue_4) (.y _returnvalue_4) _z) false false))))
  (:Started
    (if (not _bisbook)
      (bind _returnvalue_6 (Audio|CreateSound2D "/Game/Sfx/234_OutsideWalking.234_OutsideWalking" 16.0 1.0 0.0 0))
      (bind _output_get_2 (Variables|Default|SetWalking _returnvalue_6))
      (Audio|Components|Audio|Play _output_get_2 1.2)))
  (:Canceled
    (bind _walking (Variables|Default|GetWalking :!label _label)
      (:then
        (Audio|Components|Audio|Stop _walking))
      (:else)))
  (:Completed
    (goto _label)))

(event EventBeginPlay
  (bind _returnvalue (Transformation|GetActorLocation))
  (Utilities|FlowControl|Sequence
    (:then_0
      (Audio|PlaySound2D "/Game/Music/2_DivergingPath.2_DivergingPath" 2.0 1.0 0.0 0 0)
      (Audio|PlaySound2D "/Game/Sfx/2_DivergingPathAmbience.2_DivergingPathAmbience" 4.0 1.0 0.0 0 0))
    (:then_1
      (bind _returnvalue_2 (Actor|GetActorOfClass "/Game/2_Scene1/BP_Spline.BP_Spline_C"))
      (bind _output_get (Variables|Default|SetActiveSpline (Variables|/Game/2_Scene1/BP_Spline.BP_Spline_C|GetSpline _returnvalue_2)))
      (Transformation|SetActorLocation (Math|Vector|MakeVector (.x (Spline|FindLocationClosesttoWorldLocation _output_get _returnvalue "World")) (.y (Spline|FindLocationClosesttoWorldLocation _output_get _returnvalue "World")) (.Z (Math|Vector|BreakVector _returnvalue))) false false))
    (:then_2
      (Variables|Default|SetbIsBook false))))

(event EventTick
  (params (DeltaSeconds :type Float%20%28single-precision%29))
  (bind _firstpersoncamera (Variables|Default|GetFirstPersonCamera))
  (bind _returnvalue (Transformation|GetWorldLocation _firstpersoncamera))
  (bind _outhit (Collision|LineTraceForObjects _returnvalue (+ _returnvalue (* (Math|Vector|GetForwardVector _firstpersoncamera) 1e+03)) (Utilities|Array|MakeArray "ObjectTypeQuery7") true 0 "None"))
  (if (not (== (Variables|Default|GetHit%20Component) (.HitComponent (Collision|BreakHitResult _outhit))))
    (Utilities|IsValid (.HitComponent (Collision|BreakHitResult _outhit))
      (:Is%20Valid
        (CallFunction|Highlight (.HitComponent (Collision|BreakHitResult _outhit)) true))
      (:Is%20Not%20Valid
        _))
    (bind _hit_component (Variables|Default|GetHit%20Component)
      (:then
        (CallFunction|Highlight _hit_component false))
      (:else
        _))
    (Variables|Default|SetHit%20Component (.HitComponent (Collision|BreakHitResult _outhit)))))

(fn ConstructionScript)

(fn HasTag
  (params (Component :type Actor%20Component%20Object%20Reference) (Tag :type Name))
  (for _array_element (Variables|/Script/Engine.ActorComponent|GetComponentTags Component)
    (if (== _array_element Tag)
      (return true)))
  (return false))