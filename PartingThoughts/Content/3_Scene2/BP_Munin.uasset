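; BP_Munin is a highlightable character in Scene 2 that becomes detectable by queries while something overlaps its Activation volume.
; Its Highlight event toggles custom depth rendering on body, head, hair and every mesh in the Seat array.
; BeginPlay assigns the seat meshes a custom depth stencil value.
; Activation begin and end overlaps switch TraceTarget between query-only and no collision, with no filter on the overlapping actor.
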(event OnComponentBeginOverlap(Activation)
  (params (OverlappedComponent :type Primitive%20Component%20Object%20Reference) (OtherActor :type Actor%20Object%20Reference) (OtherComp :type Primitive%20Component%20Object%20Reference) (OtherBodyIndex :type Integer) (bFromSweep :type Boolean) (SweepResult :type Hit%20Result%20Structure%20%28by%20ref%29))
  (Collision|SetCollisionEnabled (Variables|Default|GetTraceTarget) "QueryOnly"))

(event OnComponentEndOverlap(Activation)
  (params (OverlappedComponent :type Primitive%20Component%20Object%20Reference) (OtherActor :type Actor%20Object%20Reference) (OtherComp :type Primitive%20Component%20Object%20Reference) (OtherBodyIndex :type Integer))
  (Collision|SetCollisionEnabled (Variables|Default|GetTraceTarget) "NoCollision"))

(event Custom|Highlight
  (params (bHighlight :type Boolean))
  (Rendering|SetRenderCustomDepth (Variables|Default|GetBody) bHighlight)
  (for _array_element (Variables|Default|GetSeat)
    (Rendering|SetRenderCustomDepth (Variables|/Script/Engine.StaticMeshActor|GetStaticMeshComponent _array_element) bHighlight)))

(event EventBeginPlay
  (for _array_element (Variables|Default|GetSeat)
    (Rendering|SetCustomDepthStencilValue (Variables|/Script/Engine.StaticMeshActor|GetStaticMeshComponent _array_element) 255)))

(fn ConstructionScript)