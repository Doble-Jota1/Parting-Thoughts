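; Scene 3 butterfly that flies along a series of splines, stopping at landing actors between them.
; Each Walk call plays a burst of flight toward the spline's first point, scaled by player distance, with random jitter and occasional drift correction.
; At spline's end it lerps to its landing; repeated Walk calls send it to the next spline.
; Timers randomize timeline-driven flapping; certain stops toggle collision and a material parameter, and custom depth provides highlighting.
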(event Custom|Walk
  (bind _returnvalue (Transformation|GetActorLocation))
  (bind _returnvalue_2 (Transformation|GetActorLocation))
  (bind _locations (Variables|Default|GetLocations))
  (bind _index (Variables|Default|GetIndex))
  (bind _wings (Variables|Default|GetWings))
  (bind _wings_2 (Variables|Default|GetWings))
  (bind _index_2 (Variables|Default|GetIndex))
  (bind _output (Utilities|Array|Get(acopy) _locations _index))
  (bind (_x _y) (Math|Vector|BreakVector _output))
  (if (Variables|Default|GetbShouldFly)
    (Utilities|FlowControl|Sequence
      (:then_0
        (Components|Timeline|SetPlayRate (Variables|Default|GetFly) 2.0)
        (bind _output_get (Variables|Default|SetFactor (Math|Float|MapRangeClamped (Math|Vector|Distance(Vector) (Transformation|GetActorLocation (Variables|Default|GetPlayer)) _returnvalue) 0.0 1e+03 1.0 2.0)))
        (CallFunction|MakeOffset)
        (bind _alpha (Timeline|Fly PlayFromStart)
          (:Update
            (Transformation|SetActorLocationAndRotation (+ _returnvalue (* 15.0 (Spline|FindDirectionClosesttoWorldLocation (Variables|Default|GetActiveSpline) _returnvalue "World") -1.0 _alpha _output_get) (Variables|Default|GetOffset)) (Math|Rotator|MakeRotfromX (Spline|FindDirectionClosesttoWorldLocation (Variables|Default|GetActiveSpline) _returnvalue "World")))
            (if (< (Math|Vector|Distance(Vector) (Spline|GetLocationatSplinePoint (Variables|Default|GetActiveSpline) 0 "World") (Spline|FindLocationClosesttoWorldLocation (Variables|Default|GetActiveSpline) (Transformation|GetActorLocation) "World")) 1e+01) :!label _label
              (Utilities|FlowControl|Sequence
                (:then_0
                  (Timeline|FlyCorrect Stop
                    (:Update
                      (Transformation|SetActorLocation (Math|Interpolation|VInterpTo _returnvalue_2 (stale _output_get_4) (Utilities|Time|GetWorldDeltaSeconds) 2.0) false false)
                      (goto _label))))
                (:then_1
                  (Timeline|Fly Stop))
                (:then_2
                  (Utilities|FlowControl|Sequence
                    (:then_0
                      (Variables|Default|SetbShouldFly false)
                      (Utilities|Time|ClearandInvalidateTimerbyHandle (Variables|Default|GetTimer))
                      (Variables|Default|SetTemp 2.0)
                      (CallFunction|Flap)
                      (if (or (== _index_2 0) (== _index_2 4))
                        (Collision|SetCollisionEnabled (Variables|Default|GetCollision) "QueryOnly")
                        (Rendering|Material|SetScalarParameterValue "/Game/4_Scene3/MPC_Toggle.MPC_Toggle" "Toggle" 1.0 :!class /Script/Engine.KismetMaterialLibrary)))
                    (:then_1
                      (Components|Timeline|SetPlayRate (Variables|Default|GetLand) 0.5)
                      (bind _output_get_2 (Variables|Default|SetStartLoc (Transformation|GetActorLocation)))
                      (bind _output_get_3 (Variables|Default|SetStartRot (Transformation|GetActorRotation)))
                      (bind _alpha_2 (Timeline|Land PlayFromStart)
                        (:Update
                          (Transformation|SetActorLocationAndRotation (Math|Vector|Lerp(Vector) _output_get_2 _output _alpha_2) (Math|Rotator|Lerp(Rotator) _output_get_3 (Math|Rotator|FindLookatRotation (Math|Vector|MakeVector _x _y 0.0) (Math|Vector|MakeVector (.X (Math|Vector|BreakVector _output_get_2)) (.Y (Math|Vector|BreakVector _output_get_2)) 0.0)) _alpha_2))
                          (Components|Timeline|SetPlayRate _wings (- (Components|Animation|GetPlayRate _wings) 0.01))))))))))
          (:Finished
            (Utilities|Time|ClearandInvalidateTimerbyHandle (Variables|Default|GetTimer))
            (if (Math|Random|RandomBoolwithWeight 0.5)
              (bind _output_get_4 (Variables|Default|SetEndLoc (Spline|FindLocationClosesttoWorldLocation (Variables|Default|GetActiveSpline) _returnvalue_2 "World")))
              (Components|Timeline|SetPlayRate (Variables|Default|GetFlyCorrect) 3.0)
              (Timeline|FlyCorrect PlayFromStart)))))
      (:then_1
        (Timeline|FlyCorrect Stop))
      (:then_2
        (bind _alpha_3 (Timeline|Depart Stop)
          (:Update
            (Transformation|SetActorLocationAndRotation (Math|Vector|Lerp(Vector) (stale _output_get_6) (Spline|GetLocationatSplinePoint (stale _output_get_5) (- (Spline|GetNumberOfSplinePoints (stale _output_get_5)) 1) "World") _alpha_3) (Math|Rotator|Lerp(Rotator) (stale _output_get_7) (Math|Rotator|FindLookatRotation (Math|Vector|MakeVector (.X (Math|Vector|BreakVector (Spline|GetLocationatSplinePoint (stale _output_get_5) (- (Spline|GetNumberOfSplinePoints (stale _output_get_5)) 1) "World"))) (.Y (Math|Vector|BreakVector (Spline|GetLocationatSplinePoint (stale _output_get_5) (- (Spline|GetNumberOfSplinePoints (stale _output_get_5)) 1) "World"))) 0.0) (Math|Vector|MakeVector (.X (Math|Vector|BreakVector (stale _output_get_6))) (.Y (Math|Vector|BreakVector (stale _output_get_6))) 0.0)) _alpha_3))
            (Components|Timeline|SetPlayRate _wings_2 (+ (Components|Animation|GetPlayRate _wings_2) 0.01)))
          (:Finished
            (Variables|Default|SetbShouldFly true)
            (Variables|Default|SetCounter 0)
            (Collision|SetCollisionEnabled (Variables|Default|GetCollision) "NoCollision")))))
    (else
      (bind _result (Math|Integer|IncrementInt (Variables|Default|GetCounter))
        (:%20%20
          (if (> _result 1)
            (Utilities|FlowControl|Sequence
              (:then_0
                (bind _result_2 (Math|Integer|IncrementInt (Variables|Default|GetIndex))
                  (:%20%20
                    (Rendering|Material|SetScalarParameterValue "/Game/4_Scene3/MPC_Toggle.MPC_Toggle" "Toggle" (Math|Conversions|ToFloat(Boolean) (or (== _result_2 0) (== _result_2 4))) :!class /Script/Engine.KismetMaterialLibrary)
                    (bind _output_get_5 (Variables|Default|SetActiveSpline (Variables|/Game/2_Scene1/BP_Spline.BP_Spline_C|GetSpline (Utilities|Array|Get(acopy) (Variables|Default|GetSplines) _result_2))))
                    (Components|Timeline|SetPlayRate (Variables|Default|GetWings) 0.0)
                    (CallFunction|Flap)
                    (bind _output_get_6 (Variables|Default|SetStartLoc (Transformation|GetActorLocation)))
                    (bind _output_get_7 (Variables|Default|SetStartRot (Transformation|GetActorRotation)))
                    (Timeline|Depart PlayFromStart))))
              (:then_1
                (Timeline|Land Stop)))))))))

(event Custom|MakeOffset
  (Utilities|FlowControl|Sequence
    (:then_0
      (Variables|Default|SetOffset (* (Math|Random|RandomUnitVector) (Math|Random|RandomFloatinRange 0.0 5.0)))
      (bind _output_get (Variables|Default|SetTemp (Math|Random|RandomFloatinRange 0.2 0.4)))
      (bind _returnvalue (Utilities|Time|SetTimerbyEvent (delegate Custom|MakeOffset) _output_get))
      (Variables|Default|SetTimer _returnvalue)
      (CallFunction|Flap))))

(event Custom|Flap
  (Utilities|FlowControl|Sequence
    (:then_0
      (Components|Timeline|SetPlayRate (Variables|Default|GetWings) (Math|Random|RandomFloatinRange 2.0 4.0))
      (bind _output_get (Variables|Default|SetLower (Math|Random|RandomFloatinRange -6e+01 -1e+01)))
      (bind _output_get_2 (Variables|Default|SetUpper (Math|Random|RandomFloatinRange 5e+01 85.0)))
      (bind _alpha (Timeline|Wings Play)
        (:Update
          (Transformation|SetRelativeRotation (Variables|Default|GetLeft) (Math|Rotator|MakeRotator (Math|Float|Lerp _output_get _output_get_2 (- 1.0 _alpha)) 0.0 0.0) false false)
          (Transformation|SetRelativeRotation (Variables|Default|GetRight) (Math|Rotator|MakeRotator (* (Math|Float|Lerp _output_get _output_get_2 (- 1.0 _alpha)) -1.0) 0.0 0.0) false false))))
    (:then_1
      (Utilities|Time|SetTimerbyEvent (delegate Custom|Stop) (Variables|Default|GetTemp)))))

(event Custom|Stop
  (bind _alpha (Timeline|Wings Stop)
    (:Update
      (Transformation|SetRelativeRotation (Variables|Default|GetLeft) (Math|Rotator|MakeRotator (Math|Float|Lerp (stale Custom|Flap _output_get) (stale Custom|Flap _output_get_2) (- 1.0 _alpha)) 0.0 0.0) false false)
      (Transformation|SetRelativeRotation (Variables|Default|GetRight) (Math|Rotator|MakeRotator (* (Math|Float|Lerp (stale Custom|Flap _output_get) (stale Custom|Flap _output_get_2) (- 1.0 _alpha)) -1.0) 0.0 0.0) false false))))

(event Custom|Highlight
  (params (bHighlight :type Boolean))
  (Rendering|SetRenderCustomDepth (Variables|Default|GetRight) bHighlight))

(event EventBeginPlay
  (bind _returnvalue (Actor|GetActorOfClass "/Game/4_Scene3/BP_PlayerScene3.BP_PlayerScene3_C"))
  (Variables|Default|SetPlayer _returnvalue)
  (bind _output_get (Variables|Default|SetActiveSpline (Variables|/Game/2_Scene1/BP_Spline.BP_Spline_C|GetSpline (Utilities|Array|Get(acopy) (Variables|Default|GetSplines)))))
  (Transformation|SetActorLocation (Spline|GetLocationatSplinePoint _output_get (- (Spline|GetNumberOfSplinePoints _output_get) 1) "World") false false)
  (for _array_element (Variables|Default|GetLandings)
    (Utilities|Array|Add (Variables|Default|GetLocations) (Transformation|GetActorLocation _array_element))))

(fn ConstructionScript)