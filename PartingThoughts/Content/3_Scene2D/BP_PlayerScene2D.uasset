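; Player actor for the 2D scene, a balancing game where the mouse slides a platform sideways beneath a ball.
; A timeline rocks the platform, its speed and amplitude building until the ball falls, then easing off.
; Once the shaking nearly stops, the ball is destroyed and the platform and scenery collapse through staggered physics activation, with the "Back"-tagged mesh released later, before Scene3 loads.
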(event EventTick
  (params (DeltaSeconds :type Float%20%28single-precision%29))
  (bind _platform (Variables|Default|GetPlatform))
  (bind _shake (Variables|Default|GetShake))
  (bind _index (Variables|Default|GetIndex))
  (bind _ball (Variables|Default|GetBall))
  (bind _returnvalue (Transformation|GetActorLocation _platform))
  (Transformation|SetActorLocation _platform (Math|Vector|MakeVector (.x _returnvalue) (Math|Float|MapRangeClamped (.y (.WorldLocation (Game|Player|ConvertMouseLocationToWorldSpace (Game|GetPlayerController 0)))) -2.5e+02 2.5e+02 -2e+02 2e+02) (.z _returnvalue)) false false)
  (Components|Timeline|SetPlayRate _shake (Math|Float|Clamp(Float) (+ (Components|Animation|GetPlayRate _shake) (Math|Float|SelectFloat -0.01 0.005 (Variables|Default|GetbDone))) 0.0 6.0))
  (bind _output_get (Variables|Default|SetShakeAmount (Math|Float|Clamp(Float) (+ (Variables|Default|GetShakeAmount) (Math|Float|SelectFloat -0.5 0.05 (Variables|Default|GetbDone))) 0.0 8e+01)))
  (bind _output_get_2 (Variables|Default|SetbDone (< (.z (Transformation|GetWorldLocation (Variables|/Game/3_Scene2D/BP_Ball.BP_Ball_C|GetSphere _ball))) -1.5e+02)))
  (if _output_get_2
    (if (Math|Float|NearlyEqual(Float) _output_get 0.0 5.0)
      (Actor|Tick|SetActorTickEnabled false)
      (Actor|DestroyActor _ball)
      (Physics|SetSimulatePhysics (Variables|/Game/3_Scene2D/BP_Platform.BP_Platform_C|GetCube (Variables|Default|GetPlatform)) true)
      (Audio|Components|Audio|Play (Variables|Default|GetMusic) 0.0)
      (Audio|PlaySound2D "/Game/Sfx/3_HeadOnShoulderVibration.3_HeadOnShoulderVibration" 1.0 1.0 0.0 0 0)
      (Utilities|FlowControl|Delay 2.0)
      (Utilities|FlowControl|Sequence
        (:then_0
          (bind _outactors (Actor|GetAllActorsOfClass "/Script/Engine.StaticMeshActor"))
          (bind _output_get_3 (Variables|Default|SetOut%20Actors _outactors))
          (if (Actor|ActorHasTag (Utilities|Array|Get(acopy) _output_get_3 _index) "Back")
            (if (not (== _index (Utilities|Array|LastIndex _output_get_3))) :!label _label
              (Math|Integer|IncrementInt _index
                (:%20%20
                  (Utilities|FlowControl|Delay (Math|Random|RandomFloatinRange 0.3 0.5))
                  (Transformation|SetMobility (Variables|/Script/Engine.StaticMeshActor|GetStaticMeshComponent (Utilities|Array|Get(acopy) _output_get_3 _index)) "Movable" :!label _label_2)
                  (Physics|SetSimulatePhysics (Variables|/Script/Engine.StaticMeshActor|GetStaticMeshComponent (Utilities|Array|Get(acopy) _output_get_3 _index)) true)
                  (goto _label))))
            (else
              (goto _label_2))))
        (:then_1
          (Utilities|FlowControl|Delay 7.0)
          (bind _outactors_2 (Actor|GetAllActorsOfClasswithTag "/Script/Engine.StaticMeshActor" "Back"))
          (Physics|SetSimulatePhysics (Variables|/Script/Engine.StaticMeshActor|GetStaticMeshComponent (Utilities|Array|Get(acopy) _outactors_2)) true)
          (Utilities|FlowControl|Delay 4.0)
          (Game|OpenLevel(byObjectReference) "/Game/4_Scene3/Scene3.Scene3"))))))

(event EventBeginPlay
  (Utilities|FlowControl|Sequence
    (:then_0
      (bind _returnvalue (Actor|GetActorOfClass "/Game/3_Scene2D/BP_Ball.BP_Ball_C"))
      (Variables|Default|SetBall _returnvalue)
      (bind _returnvalue_2 (Actor|GetActorOfClass "/Game/3_Scene2D/BP_Platform.BP_Platform_C"))
      (Variables|Default|SetPlatform _returnvalue_2)
      (bind _alpha (Timeline|Shake Play)
        (:Update
          (Transformation|SetActorRotation (Variables|Default|GetPlatform) (Math|Rotator|MakeRotator (* _alpha (Variables|Default|GetShakeAmount)) 0.0 0.0)))))
    (:then_1
      (bind _returnvalue_3 (Audio|CreateSound2D "/Game/Music/3_HeadOnShoulderLoop.3_HeadOnShoulderLoop" 1.0 1.0 0.0 0))
      (bind _output_get (Variables|Default|SetMusic _returnvalue_3))
      (Audio|Components|Audio|Play _output_get 0.0))))

(fn ConstructionScript)