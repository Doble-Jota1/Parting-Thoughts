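; BP_PartingGameInstance is a game instance that handles level transitions with a white screen fade and creates 2D sounds.
; LoadLevel fades out, waits for the fade to finish, opens the level by object reference, then after a brief delay fades in.
; FadeOut and FadeIn drive the first player's camera manager fade, holding when finished.
; CreateSound wraps CreateSound2D with a volume multiplier and returns the result.
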(event Custom|FadeIn
  (params (Duration :type Float%20%28single-precision%29))
  (CameraFades|StartCameraFade (Game|GetPlayerCameraManager 0) 1.0 0.0 Duration "(R=1.000000,G=1.000000,B=1.000000,A=1.000000)" false true))

(event Custom|LoadLevel
  (params (Level :type World%20Soft%20Object%20Reference))
  (CallFunction|FadeOut 2.0)
  (Utilities|FlowControl|Delay 2.0)
  (Game|OpenLevel(byObjectReference) Level)
  (Utilities|FlowControl|Delay 0.01)
  (CallFunction|Fadein 3.0))

(event Custom|FadeOut
  (params (Duration :type Float%20%28single-precision%29))
  (CameraFades|StartCameraFade (Game|GetPlayerCameraManager 0) 0.0 1.0 Duration "(R=1.000000,G=1.000000,B=1.000000,A=1.000000)" false true))

(fn CreateSound
  (params (Sound :type Sound%20Base%20Object%20Reference) (VolumeMultiplier :type Float%20%28single-precision%29))
  (bind _returnvalue (Audio|CreateSound2D Sound VolumeMultiplier 1.0 0.0 0 true))
  (return _returnvalue))