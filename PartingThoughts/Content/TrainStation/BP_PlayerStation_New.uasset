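; Player pawn for the train station scene: a spline-guided walk into a scripted parting, then a ticket choice in a book.
; Timelines drive the post-process intro fade and camera moves, while delayed sequences time music, frozen Niagara effects and title-card dialogue.
; Holding Space walks the spline until Parting fires and later spawns the book.
; Mouse traces reveal hovered book components; clicking one tagged Empty loads FractalPath, others show a rejection card.
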(event Custom|ShowBook
  (bind _returnvalue (Transformation|GetActorForwardVector))
  (bind _sphere (Variables|Default|GetSphere))
  (bind _returnvalue_2 (Transformation|GetWorldTransform _sphere))
  (bind _returnvalue_3 (* _returnvalue 1e+02))
  (bind _returnvalue_4 (- (.location _returnvalue_2) "0.000000,0.000000,100.000000"))
  (bind _returnvalue_5 (- _returnvalue_4 _returnvalue_3))
  (Variables|Default|SetbIsBook true)
  (bind _returnvalue_6 (Game|SpawnActorfromClass "/Game/TrainStation/BP_Book.BP_Book_C" (Math|Transform|MakeTransform _returnvalue_5 "0, 0, 0" "0.060000,0.060000,0.060000") "AlwaysSpawn" "MultiplyWithRoot" 0 0))
  (bind _output_get (Variables|Default|SetBook _returnvalue_6))
  (Transformation|AttachComponentToComponent _output_get (Variables|Default|GetSphere) "None" "KeepWorld" "KeepRelative" "KeepWorld" true)
  (bind _alpha (Timeline|BookTakeOut PlayFromStart)
    (:Update
      (Transformation|SetActorLocation (Variables|Default|GetBook) (Math|Vector|Lerp(Vector) _returnvalue_5 (.location _returnvalue_2) _alpha) false false))
    (:Finished
      (Utilities|FlowControl|Sequence
        (:then_0
          (Utilities|FlowControl|Delay 3.2)
          (Variables|Default|SetbBookTrace true)
          (Variables|/Script/Engine.PlayerController|SetbShowMouseCursor (Game|GetPlayerController 0) true))
        (:then_1
          (Utilities|FlowControl|Delay 1.0)
          (Default|StartShake (Variables|Default|GetBook)))))))

(event Custom|BookTrace
  (bind _returnvalue (Game|GetPlayerController 0))
  (bind (_worldlocation _worlddirection) (Game|Player|ConvertMouseLocationToWorldSpace _returnvalue))
  (bind _outhit (Collision|LineTraceForObjects _worldlocation (+ _worldlocation (* _worlddirection 5e+02)) (Utilities|Array|MakeArray "ObjectTypeQuery8") true 0 "None"))
  (if (not (== (Variables|Default|GetHit%20Component) (.HitComponent (Collision|BreakHitResult _outhit))))
    (Utilities|IsValid (.HitComponent (Collision|BreakHitResult _outhit))
      (:Is%20Valid
        (Development|SetHiddeninGame (.HitComponent (Collision|BreakHitResult _outhit)) false false))
      (:Is%20Not%20Valid
        _))
    (bind _hit_component (Variables|Default|GetHit%20Component)
      (:then
        (Development|SetHiddeninGame _hit_component true false))
      (:else
        _))
    (bind _output_get (Variables|Default|SetHit%20Component (.HitComponent (Collision|BreakHitResult _outhit))))))

(event Custom|RaiseArm
  (Utilities|FlowControl|Sequence
    (:then_0
      (bind _alpha (Timeline|Raise PlayFromStart)
        (:Update
          (Transformation|SetRelativeLocationAndRotation (Variables|Default|GetLiftingArm) (Math|Vector|Lerp(Vector) "0.300000,13.000000,-27.000000" "27.000000,14.000000,-13.000000" _alpha) (Math|Rotator|Lerp(Rotator) "0.700000,-99.000000,-19.000000" "13.500000,-105.000000,-18.000000" _alpha true) false false))))
    (:then_1
      (Utilities|FlowControl|Delay 1.25)
      (Variables|Default|SetbRaiseArm true))))

(event Custom|Rainbow
  (Utilities|Struct|SetmembersinPostProcessSettings (Variables|/Script/Engine.PostProcessVolume|GetSettings (Variables|Default|GetPP)) (.OutItem (Utilities|Array|Random (Variables|Default|GetRainbows))))
  (Utilities|Time|SetTimerbyEvent (delegate Custom|Rainbow) (Math|Random|RandomFloatinRange 2.0 5.0)))

(event Custom|Parting
  (bind _returnvalue (Transformation|GetActorLocation))
  (bind _returnvalue_2 (Game|GetPlayerController 0))
  (bind _titlecard (Variables|Default|GetTitleCard))
  (bind _firstpersoncamera (Variables|Default|GetFirstPersonCamera))
  (Variables|Default|SetbIsBook true)
  (Utilities|FlowControl|Sequence
    (:then_0
      (bind _output_get (Variables|Default|SetStartingRotation (Pawn|GetControlRotation _returnvalue_2 :!class /Script/Engine.Controller)))
      (bind _alpha (Timeline|Orient PlayFromStart)
        (:Update
          (Pawn|SetControlRotation _returnvalue_2 (Math|Rotator|Lerp(Rotator) _output_get "3.500000,-12.000000,0.000000" _alpha true)))))
    (:then_1
      (Audio|Components|Audio|FadeOut (Variables|Default|GetMusic) 6.0 0.0 "Linear" :!class /Script/Engine.AudioComponent)
      (bind _returnvalue_3 (Default|CreateSound (Variables|Default|GetGameInstance) "/Game/Music/1_TrainStation_Slowed.1_TrainStation_Slowed" 1.0))
      (bind _output_get_2 (Variables|Default|SetMusic2 _returnvalue_3))
      (Audio|Components|Audio|FadeIn _output_get_2 6.0 1.0 0.0 "Linear" :!class /Script/Engine.AudioComponent))
    (:then_2
      (Utilities|FlowControl|Delay 1.0)
      (bind _output_get_3 (Variables|Default|SetTemp (Variables|/Script/Engine.CameraComponent|GetFieldOfView _firstpersoncamera)))
      (Variables|Default|SetLocationTemp _returnvalue)
      (bind _alpha_2 (Timeline|Zoom PlayFromStart)
        (:Update
          (Camera|SetFieldOfView _firstpersoncamera (Math|Float|Lerp _output_get_3 88.0 _alpha_2))
          (Transformation|SetActorLocation (Math|Vector|Lerp(Vector) (Variables|Default|GetLocationTemp) (Math|Vector|MakeVector 4326.0 788.0 (.Z (Math|Vector|BreakVector _returnvalue))) _alpha_2) false false))))
    (:then_3
      (Utilities|FlowControl|Delay 1.0)
      (CallFunction|RaiseArm)
      (Utilities|FlowControl|Delay 2.4)
      (Audio|Components|Audio|FadeOut (Variables|Default|GetAmbience) 0.3 0.0 "Linear" :!class /Script/Engine.AudioComponent)
      (bind _outactors (Actor|GetAllActorsOfClass "/Script/Niagara.NiagaraActor"))
      (for _array_element _outactors
        (Class|NiagaraComponent|SetPaused (Variables|/Script/Niagara.NiagaraActor|GetNiagaraComponent _array_element) true))
      (Utilities|FlowControl|Delay 5.0)
      (CallFunction|NextCard "I RAISE MY HAND 
\"Wait\"")
      (Utilities|FlowControl|Delay 0.1)
      (UserInterface|Viewport|AddtoViewport _titlecard 0)
      (Utilities|FlowControl|Delay 4.0)
      (CallFunction|NextCard "\"Why don't you come with me\" 
She says")
      (Utilities|FlowControl|Delay 4.0)
      (CallFunction|NextCard "\"I don't have the ticket\" 
I check my collection once more")
      (Utilities|FlowControl|Delay 4.0)
      (Widget|RemovefromParent _titlecard)
      (Audio|Components|Audio|Stop (Variables|Default|GetCardSfx))
      (Utilities|FlowControl|Sequence
        (:then_0
          (bind _output_get_4 (Variables|Default|SetAnotherTemp (Transformation|GetActorLocation)))
          (bind _alpha_3 (Timeline|ZoomOut PlayFromStart)
            (:Update
              (Transformation|SetActorLocation (Math|Vector|Lerp(Vector) _output_get_4 (Variables|Default|GetLocationTemp) _alpha_3) false false))))
        (:then_1
          (Utilities|FlowControl|Delay 5.0)
          (CallFunction|ShowBook))))))

(event Custom|NextCard
  (params (InText :type Text))
  (bind _returnvalue (Audio|CreateSound2D "/Game/Sfx/Card.Card" 1.0 1.0 0.0 0))
  (bind _output_get (Variables|Default|SetCardSfx _returnvalue))
  (Audio|Components|Audio|Play _output_get 0.0)
  (Utilities|FlowControl|Delay 0.05)
  (Rendering|Components|TextRender|SetText (Variables|/Game/TrainStation/WB_TitleCard.WB_TitleCard_C|GetText (Variables|Default|GetTitleCard)) InText))

(event Custom|IntroFade
  (Variables|Default|SetbIsBook true)
  (Utilities|FlowControl|Sequence
    (:then_0
      (bind _returnvalue (Actor|GetActorOfClass "/Script/Engine.PostProcessVolume"))
      (bind _output_get (Variables|Default|SetPP _returnvalue))
      (Components|Timeline|SetPlayRate (Variables|Default|GetIntro) 0.1)
      (bind _output_get_2 (Variables|Default|SetExposure (.AutoExposureBias (Utilities|Struct|BreakPostProcessSettings (Variables|/Script/Engine.PostProcessVolume|GetSettings _output_get)))))
      (bind _output_get_3 (Variables|Default|SetFocalDistance (.DepthOfFieldFocalDistance (Utilities|Struct|BreakPostProcessSettings (Variables|/Script/Engine.PostProcessVolume|GetSettings _output_get)))))
      (bind _alpha (Timeline|Intro PlayFromStart)
        (:Update
          (Utilities|Struct|SetmembersinPostProcessSettings (Variables|/Script/Engine.PostProcessVolume|GetSettings _output_get) (Math|Float|Lerp 21.0 _output_get_2 (Math|Float|Clamp(Float) (* _alpha 3.0))) (Math|Float|Lerp 0.99 _output_get_3 _alpha) (Utilities|Struct|MakeWeightedBlendables (Utilities|Array|MakeArray (Utilities|Struct|MakeWeightedBlendable (Math|Float|Lerp 1.0 0.1 _alpha) "/Game/TrainStation/PP_Train1.PP_Train1")))))))
    (:then_1
      (Utilities|FlowControl|Delay 5.0)
      (Variables|Default|SetbIsBook false))))

(event Input|EnhancedActionEvents|EnhancedInputActionIA_Space
  (params (ActionValue :type Boolean) (ElapsedSeconds :type Float%20%28double-precision%29) (TriggeredSeconds :type Float%20%28double-precision%29) (InputAction :type Input%20Action%20Object%20Reference :default "/Game/Blueprints/Input/IA_Space.IA_Space"))
  (bind _returnvalue (Transformation|GetActorLocation))
  (bind _bisbook (Variables|Default|GetbIsBook))
  (:Triggered
    (if (not _bisbook)
      (Pawn|Input|AddMovementInput (Spline|FindDirectionClosesttoWorldLocation (Variables|Default|GetSpline) _returnvalue "World") -0.8 false)
      (Audio|PlaySound2D 0 1.0 1.0 0.0 0 0)
      (if (< (Class|KismetMathLibrary|VectorDistanceSquared (Variables|Default|GetDestination) _returnvalue) (Variables|Default|GetThreshold))
        (CallFunction|Parting))))
  (:Started
    (if (not _bisbook)
      (bind _returnvalue_2 (Audio|CreateSound2D "/Game/Sfx/15_PlatformWalking.15_PlatformWalking" 1.25 1.0 0.0 0))
      (bind _output_get (Variables|Default|SetWalking _returnvalue_2))
      (Audio|Components|Audio|Play _output_get (.OutItem (Utilities|Array|Random (Variables|Default|GetWalkTimes))))))
  (:Canceled
    (bind _walking (Variables|Default|GetWalking :!label _label)
      (:then
        (Audio|Components|Audio|Stop _walking))
      (:else)))
  (:Completed
    (goto _label)))

(event Input|EnhancedActionEvents|EnhancedInputActionIA_LeftClick
  (params (ActionValue :type Boolean) (ElapsedSeconds :type Float%20%28double-precision%29) (TriggeredSeconds :type Float%20%28double-precision%29) (InputAction :type Input%20Action%20Object%20Reference :default "/Game/Blueprints/Input/IA_LeftClick.IA_LeftClick"))
  (bind _titlecard (Variables|Default|GetTitleCard))
  (:Completed
    (if (Variables|Default|GetbBookTrace)
      (bind _hit_component (Variables|Default|GetHit%20Component)
        (:then
          (bind _bhastag (CallFunction|HasTag _hit_component "Empty"))
          (if _bhastag
            (Utilities|FlowControl|Sequence
              (:then_0
                (Utilities|FlowControl|Delay 3.0)
                (bind _asbp_parting_game_instance (Utilities|Casting|CastToBP_PartingGameInstance (Game|GetGameInstance)))
                (Default|LoadLevel _asbp_parting_game_instance "/Game/Scene1/FractalPath.FractalPath"))
              (:then_1
                (Audio|PlaySound2D "/Game/Sfx/1_Swell.1_Swell" 1.0 1.0 0.0 0 0)))
            (else
              (Variables|Default|SetbBookTrace false)
              (CallFunction|NextCard "\"But this ticket is unprinted\" 
She says")
              (UserInterface|Viewport|AddtoViewport _titlecard 0)
              (Utilities|FlowControl|Delay 4.0)
              (Widget|RemovefromParent _titlecard)
              (Audio|Components|Audio|Stop (Variables|Default|GetCardSfx))
              (Variables|Default|SetbBookTrace true))))
        (:else)))))

(event Input|EnhancedActionEvents|EnhancedInputActionIA_Look
  (params (ActionValue :type Vector%202D%20Structure) (ElapsedSeconds :type Float%20%28double-precision%29) (TriggeredSeconds :type Float%20%28double-precision%29) (InputAction :type Input%20Action%20Object%20Reference :default "/Game/Blueprints/Input/IA_Look.IA_Look"))
  (if (not (Variables|Default|GetbIsBook))
    (Pawn|Input|AddControllerYawInput (.x ActionValue))
    (Pawn|Input|AddControllerPitchInput (.y ActionValue))))

(event Input|EnhancedActionEvents|EnhancedInputActionIA_Esc
  (params (ActionValue :type Boolean) (ElapsedSeconds :type Float%20%28double-precision%29) (TriggeredSeconds :type Float%20%28double-precision%29) (InputAction :type Input%20Action%20Object%20Reference :default "/Game/Blueprints/Input/IA_Esc.IA_Esc")))

(event EventBeginPlay
  (bind _returnvalue (Transformation|GetActorLocation))
  (Utilities|FlowControl|Sequence
    (:then_0
      (bind _returnvalue_2 (Actor|GetActorOfClass "/Game/Scene1/BP_Spline.BP_Spline_C"))
      (bind _output_get (Variables|Default|SetSpline (Variables|/Game/Scene1/BP_Spline.BP_Spline_C|GetSpline _returnvalue_2)))
      (Transformation|SetActorLocation (Math|Vector|MakeVector (.x (Spline|FindLocationClosesttoWorldLocation _output_get _returnvalue "World")) (.y (Spline|FindLocationClosesttoWorldLocation _output_get _returnvalue "World")) (.Z (Math|Vector|BreakVector _returnvalue))) false false)
      (Variables|Default|SetDestination (Spline|GetLocationatSplinePoint _output_get 0 "World"))
      (CallFunction|IntroFade))
    (:then_1
      (bind _returnvalue_3 (UserInterface|CreateWidget "/Game/TrainStation/WB_TitleCard.WB_TitleCard_C"))
      (Variables|Default|SetTitleCard _returnvalue_3))
    (:then_2
      (bind _asbp_parting_game_instance (Utilities|Casting|CastToBP_PartingGameInstance (Game|GetGameInstance)))
      (bind _output_get_2 (Variables|Default|SetGameInstance _asbp_parting_game_instance))
      (bind _returnvalue_4 (Default|CreateSound _output_get_2 "/Game/Music/1_TrainStation_Original.1_TrainStation_Original" 2.5))
      (bind _output_get_3 (Variables|Default|SetMusic _returnvalue_4))
      (Audio|Components|Audio|FadeIn _output_get_3 5.0 1.0 1.0 "Linear" :!class /Script/Engine.AudioComponent)
      (Utilities|FlowControl|Delay 3.0)
      (bind _returnvalue_5 (Default|CreateSound _output_get_2 "/Game/Sfx/1_TrainStationAmbience.1_TrainStationAmbience" 1.0))
      (bind _output_get_4 (Variables|Default|SetAmbience _returnvalue_5))
      (Audio|Components|Audio|FadeIn _output_get_4 6.0 1.0 0.0 "Linear" :!class /Script/Engine.AudioComponent))))

(event EventTick
  (params (DeltaSeconds :type Float%20%28single-precision%29))
  (Utilities|FlowControl|Sequence
    (:then_0
      (if (Variables|Default|GetbBookTrace)
        (CallFunction|BookTrace)))))

(fn ConstructionScript)

(fn HasTag
  (params (Component :type Actor%20Component%20Object%20Reference) (Tag :type Name))
  (for _array_element (Variables|/Script/Engine.ActorComponent|GetComponentTags Component)
    (if (== _array_element Tag)
      (return true)))
  (return false))