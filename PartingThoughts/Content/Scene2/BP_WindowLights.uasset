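; BP_WindowLights is an actor that scrolls its rect lights along world Y, likely as moving coloured light for windows in Scene2.
; BeginPlay gathers every RectLightComponent and gives each a random speed.
; Tick moves each light toward negative Y by a per-frame step, not scaled by delta time.
; Lights passing the lower bound jump back by a fixed distance and receive a new random speed and fully saturated hue.
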(event EventTick
  (params (DeltaSeconds :type Float%20%28single-precision%29))
  (for (_array_element _array_index) (Variables|Default|GetLights)
    (Transformation|AddWorldOffset _array_element (* (Math|Vector|MakeVector 0.0 -1.0 0.0) (Utilities|Array|Get(acopy) (Variables|Default|GetSpeed) _array_index)) false false)
    (if (> -9e+02 (.y (Transformation|GetWorldLocation _array_element)))
      (Transformation|AddWorldOffset _array_element "0.000000,1400.000000,0.000000" false false)
      (Utilities|Array|SetArrayElem (Variables|Default|GetSpeed) _array_index (Math|Random|RandomFloatinRange 1.0 4.0))
      (Rendering|Components|Light|SetLightColor _array_element (Class|KismetMathLibrary|HSVtoRGB (Math|Random|RandomFloatinRange 0.0 3.6e+02) 1.0 1.0 1.0) true))))

(event EventBeginPlay
  (bind _output_get (Variables|Default|SetLights (Actor|GetComponentsByClass "/Script/Engine.RectLightComponent")))
  (for _array_element _output_get
    (Utilities|Array|Add (Variables|Default|GetSpeed) (Math|Random|RandomFloatinRange 1.0 4.0))))

(fn ConstructionScript)