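; BP_Jerry is a Scene2 actor that runs a timed Chaos destruction setup on its Geometry Collection.
; Four seconds after BeginPlay it spawns an anchor field at an offset below the actor and writes it into the collection's InitializationFields.
; It then spawns an FS_MasterField_Child field above the actor and, after a short delay, enables physics simulation on the collection.
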(event EventBeginPlay
  (bind _returnvalue (Transformation|GetActorLocation))
  (Utilities|FlowControl|Delay 4.0)
  (bind _returnvalue_2 (Game|SpawnActorfromClass "/Engine/EditorResources/FieldNodes/FS_AnchorField_Generic.FS_AnchorField_Generic_C" (Math|Transform|MakeTransform (- _returnvalue "32.000000,-32.000000,45.000000") "0, 0, 0" "1.000000,1.000000,1.000000") "AlwaysSpawn" "MultiplyWithRoot" 0 0))
  (bind _output_get (Variables|Default|SetAnchor _returnvalue_2))
  (Utilities|Array|SetArrayElem (Variables|/Script/GeometryCollectionEngine.GeometryCollectionComponent|GetInitializationFields (Variables|Default|GetGeometryCollection)) 0 _output_get true)
  (Game|SpawnActorfromClass "/Game/Scene2/Fracture/FS_MasterField_Child.FS_MasterField_Child_C" (Math|Transform|MakeTransform (+ _returnvalue "5.000000,-11.000000,200.000000") "0, 0, 0" "1.000000,1.000000,1.000000") "AlwaysSpawn" "MultiplyWithRoot" 0 0)
  (Utilities|FlowControl|Delay 0.2)
  (Physics|SetSimulatePhysics (Variables|Default|GetGeometryCollection) true))

(fn ConstructionScript)