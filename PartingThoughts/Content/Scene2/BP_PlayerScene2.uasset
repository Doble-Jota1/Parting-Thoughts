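; Scene 2 first-person player that walks a rail along the level's BP_Spline while Space is held, with free look.
; Movement follows the spline direction, easing slower when a lookahead dot product detects a bend, and wraps to the start near the end.
; BeginPlay starts music and ambience, and Space drives footstep audio.
; Tick prints camera-trace hits for debugging; an IsBook camera pan is left unconnected.
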(event Input|EnhancedActionEvents|EnhancedInputActionIA_Space
  (params (ActionValue :type Boolean) (ElapsedSeconds :type Float%20%28double-precision%29) (TriggeredSeconds :type Float%20%28double-precision%29) (InputAction :type Input%20Action%20Object%20Reference :default "/Game/Blueprints/Input/IA_Space.IA_Space"))
  (bind _returnvalue (Transformation|GetActorLocation))
  (bind _returnvalue_2 (Transformation|GetActorLocation))
  (bind _bisbook (Variables|Default|GetbIsBook))
  (bind _activespline (Variables|Default|GetActiveSpline))
  (bind _returnvalue_3 (Spline|FindDirectionClosesttoWorldLocation _activespline _returnvalue "World"))
  (bind _returnvalue_4 (Spline|GetLocationatSplinePoint _activespline 0 "World"))
  (bind _z (Math|Vector|BreakVector _returnvalue_2))
  (bind _returnvalue_5 (Spline|FindLocationClosesttoWorldLocation _activespline _returnvalue "World"))
  (:Triggered
    (if (not _bisbook)
      (Transformation|SetActorLocation (Math|Vector|MakeVector (.x _returnvalue_5) (.y _returnvalue_5) _z) false false)
      (bind _output_get (Variables|Default|SetCurrentSpeed (Math|Interpolation|FInterpTo (stale _output_get) (Math|Float|SelectFloat 0.05 0.3 (< (/ (+ (Math|Vector|DotProduct _returnvalue_3 (Spline|GetDirectionatDistanceAlongSpline _activespline (+ (Class|SplineComponent|GetDistanceAlongSplineatLocation _activespline _returnvalue "World") (Variables|Default|GetLookahead)) "World")) 1.0) 2.0) 0.7)) (Utilities|Time|GetWorldDeltaSeconds) 4.0)))
      (Pawn|Input|AddMovementInput _returnvalue_3 _output_get false)
      (if (not (> (Class|KismetMathLibrary|VectorDistanceSquared (Spline|GetLocationatSplinePoint _activespline (Spline|GetNumberOfSplinePoints _activespline) "World") _returnvalue_2) 8e+03))
        (Transformation|SetActorLocation (Math|Vector|MakeVector (.x _returnvalue_4) (.y _returnvalue_4) _z) false false))))
  (:Started
    (if (not _bisbook)
      (bind _returnvalue_6 (Audio|CreateSound2D "/Game/Sfx/234_OutsideWalking.234_OutsideWalking" 16.0 1.0 0.0 0))
      (bind _output_get_2 (Variables|Default|SetWalking _returnvalue_6))
      (Audio|Components|Audio|Play _output_get_2 1.2)))
  (:Canceled
    (bind _walking (Variables|Default|GetWalking :!label _label)
      (:then
        (Audio|Components|Audio|Stop _walking))
      (:else)))
  (:Completed
    (goto _label)))

(event Input|EnhancedActionEvents|EnhancedInputActionIA_Look
  (params (ActionValue :type Vector%202D%20Structure) (ElapsedSeconds :type Float%20%28double-precision%29) (TriggeredSeconds :type Float%20%28double-precision%29) (InputAction :type Input%20Action%20Object%20Reference :default "/Game/Blueprints/Input/IA_Look.IA_Look"))
  (if (not (Variables|Default|GetbIsBook))
    (Pawn|Input|AddControllerYawInput (.x ActionValue))
    (Pawn|Input|AddControllerPitchInput (.y ActionValue))))

(event EventBeginPlay
  (bind _returnvalue (Transformation|GetActorLocation))
  (Utilities|FlowControl|Sequence
    (:then_0
      (Audio|PlaySound2D "/Game/Music/2_DivergingPath.2_DivergingPath" 2.0 1.0 0.0 0 0)
      (Audio|PlaySound2D "/Game/Sfx/2_DivergingPathAmbience.2_DivergingPathAmbience" 4.0 1.0 0.0 0 0))
    (:then_1
      (bind _returnvalue_2 (Actor|GetActorOfClass "/Game/Scene1/BP_Spline.BP_Spline_C"))
      (bind _output_get (Variables|Default|SetActiveSpline (Variables|/Game/Scene1/BP_Spline.BP_Spline_C|GetSpline _returnvalue_2)))
      (Transformation|SetActorLocation (Math|Vector|MakeVector (.x (Spline|FindLocationClosesttoWorldLocation _output_get _returnvalue "World")) (.y (Spline|FindLocationClosesttoWorldLocation _output_get _returnvalue "World")) (.Z (Math|Vector|BreakVector _returnvalue))) false false))
    (:then_2
      (Variables|Default|SetbIsBook false))))

(event EventTick
  (params (DeltaSeconds :type Float%20%28single-precision%29))
  (bind _firstpersoncamera (Variables|Default|GetFirstPersonCamera))
  (bind _returnvalue (Transformation|GetWorldLocation _firstpersoncamera))
  (bind (_outhit _returnvalue_2) (Collision|LineTraceForObjects _returnvalue (+ _returnvalue (* (Math|Vector|GetForwardVector _firstpersoncamera) 1e+03)) (Utilities|Array|MakeArray "ObjectTypeQuery7") true 0 "None"))
  (if _returnvalue_2
    (Development|PrintString (Utilities|GetDisplayName (.HitActor (Collision|BreakHitResult _outhit))))))

(fn ConstructionScript)

(fn HasTag
  (params (Component :type Actor%20Component%20Object%20Reference) (Tag :type Name))
  (for _array_element (Variables|/Script/Engine.ActorComponent|GetComponentTags Component)
    (if (== _array_element Tag)
      (return true)))
  (return false))