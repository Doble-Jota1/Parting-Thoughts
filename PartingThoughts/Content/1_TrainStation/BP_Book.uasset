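; BP_Book is an animated book actor for the train station that plays its opening on begin play and can float with a subtle shake.
; BeginPlay rewinds the cover and page meshes, then starts their animations with staggered delays.
; StartShake records the origin, enables Tick and starts a self-rescheduling random timer.
; Each Jitter picks a nearby offset or occasionally the origin, and Tick slowly interpolates toward it.
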(event Custom|Jitter
  (Utilities|Time|SetTimerbyEvent (delegate Custom|Jitter) (Math|Random|RandomFloatinRange 0.4 0.6))
  (if (> (Math|Random|RandomFloat) 0.2)
    (Variables|Default|SetTarget (+ (Transformation|GetActorLocation) (* (Math|Random|RandomUnitVector) (Math|Random|RandomFloatinRange 4.0 6.0))))
    (else
      (Variables|Default|SetTarget (Variables|Default|GetStart)))))

(event Custom|StartShake
  (Variables|Default|SetStart (Transformation|GetActorLocation))
  (CallFunction|Jitter)
  (Actor|Tick|SetActorTickEnabled true))

(event EventTick
  (params (DeltaSeconds :type Float%20%28single-precision%29))
  (Transformation|SetActorLocation (Math|Interpolation|VInterpTo (Transformation|GetActorLocation) (Variables|Default|GetTarget) DeltaSeconds 0.2) false false))

(event EventBeginPlay
  (Components|Animation|SetPosition (Variables|Default|GetInitialPage) 0.0 false)
  (Utilities|FlowControl|Delay 1.1)
  (Components|Animation|PlayAnimation (Variables|Default|GetSkeletalMesh) "/Game/1_TrainStation/Book/BookOuter_Skeleton_Sequence.BookOuter_Skeleton_Sequence" false)
  (Utilities|FlowControl|Delay 0.1)
  (Audio|Components|Audio|Play (Variables|Default|GetInitialPage) false)
  (Utilities|FlowControl|Delay 0.1)
  (Audio|Components|Audio|Play (Variables|Default|GetInitialPage1) false)
  (Utilities|FlowControl|Sequence
    (:then_0
      (Utilities|FlowControl|Delay 0.2)
      (Audio|Components|Audio|Play (Variables|Default|GetPage1) false)
      (Utilities|FlowControl|Delay 0.1)
      (Audio|Components|Audio|Play (Variables|Default|GetPage2) false)
      (Utilities|FlowControl|Delay 0.15)
      (Audio|Components|Audio|Play (Variables|Default|GetPage3) false))
    (:then_1
      (Utilities|FlowControl|Delay 0.05)
      (Audio|Components|Audio|Play (Variables|Default|GetRightPage1) false))))

(fn ConstructionScript)