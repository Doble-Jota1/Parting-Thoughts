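; BP_Column is a train station set-dressing actor that generates a row of column meshes with randomized proportions.
; Its construction script adds a static mesh component per index from zero through NumColumns inclusive, stepping along the actor's right vector by Spacing.
; Random factors vary Height, Width (shared by X and Y) and spacing, with spacing jitter growing along the row.
; Unseeded randomness re-rolls the layout whenever construction reruns.
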(event EventBeginPlay)

(event Collision|EventActorBeginOverlap
  (params (OtherActor :type Actor%20Object%20Reference)))

(event EventTick
  (params (DeltaSeconds :type Float%20%28single-precision%29)))

(fn ConstructionScript
  (for _index (range 0 (Variables|Default|GetNumColumns))
    (bind _returnvalue (AddComponent|AddStaticMeshComponent false))
    (Components|StaticMesh|SetStaticMesh _returnvalue "/Game/TrainStation/Column.Column")
    (bind _output_get (LocalVariables|SettEMP (* (Variables|Default|GetWidth) (Math|Random|RandomFloatinRange 0.8 1.2))))
    (Transformation|SetWorldTransform _returnvalue (Math|Transform|MakeTransform (+ (* _index (Transformation|GetActorRightVector) (* (Variables|Default|GetSpacing) (Math|Random|RandomFloatinRange 0.9 1.1))) (Transformation|GetActorLocation)) "0, 0, 0" (Math|Vector|MakeVector _output_get _output_get (* (Variables|Default|GetHeight) (Math|Random|RandomFloatinRange 0.6 1.8)))) false false)))